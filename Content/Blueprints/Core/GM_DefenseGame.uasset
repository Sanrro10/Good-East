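; Game mode for a boat defense game that spawns waves of enemy boats.
; On BeginPlay it loads spawn rows from a data table and sets a looping timer that advances the wave number.
; Each wave spawns that wave's boats at registered spawners with matching IDs, then has their AI controllers move them to set destinations.
; Helper functions return a boat and hand out successive avoidance groups from arrays.
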(event `self.ReceiveBeginPlay`
  (bind _spawnerdt (`self.SpawnerDT`))
  ;[1 0 0.09375] GetDatatableInfo
  (bind _outrownames (`DataTableFunctionLibrary.GetDataTableRowNames` _spawnerdt))
  (for _array_element _outrownames
    (bind _returnvalue (`|GetDataTableRow` _spawnerdt _array_element)
      (:`then`
        (`KismetArrayLibrary.Array_Add` (`self.BoatStructs`) _returnvalue)
        (`KismetSystemLibrary.K2_SetTimerDelegate` (delegate `New Wave`) 5.0 true)))))

(event `New Wave`
  (`/Engine/EditorBlueprintResources/StandardMacros.IncrementInt` (`self.WaveNumber`)
    (:`  `
      (`self.StartWave`))))

(fn `Add Spawner`
  (params (BoatSpawner :type "/Game/Blueprints/Core/Boats/BP_BoatSpawner Object Reference"))
  (`KismetArrayLibrary.Array_Add` (`self.Spawners`) BoatSpawner))

(fn `Get Avoidance Group ID`
  (returns (AvoidanceGroup :type "NavAvoidanceMask Structure") (GroupsToAvoid :type "NavAvoidanceMask Structure"))
  (locals (GroupsToAvoidArray :type "Array of NavAvoidanceMask Structure") (AvoidanceGroupArray :type "Array of NavAvoidanceMask Structure"))
  (`/Engine/EditorBlueprintResources/StandardMacros.IncrementInt` (`self.CurrentGroup ID`)
    (:`  `
      (return (`|GetArrayItem` (`local.AvoidanceGroupArray`) (`self.CurrentGroup ID`)) (`|GetArrayItem` (`local.GroupsToAvoidArray`) (`self.CurrentGroup ID`))))))

(fn `GetEnemyFromPool`
  (returns (Boat :type "/Game/Blueprints/Core/Boats/BP_Boat Class Reference"))
  (return "/Game/Blueprints/Core/Boats/BP_Boat.BP_Boat_C"))

(fn `StartWave`
  (locals (CurrentSpawnerID :type Integer) (CurrentBoatType :type "/Game/Structures+Enumerators/EBoatType Enum") (CurrentBoatDestination :type "Vector Structure"))
  ;[0.5938 0 1] Setting each variable of a boat to be spawned
  (for _array_element (`self.BoatStructs`)
    (bind (_spawnerid _wavenumber _boat _destination) (break `/Game/Structures+Enumerators/SBoatSpawner` _array_element))
    (set `local.CurrentSpawnerID` _spawnerid)
    (set `local.CurrentBoatType` _boat)
    (set `local.CurrentBoatDestination` _destination)
    ;[0.06965 1 0] Checks if the boat's wave matches the current wave
    (if (== _wavenumber (`self.WaveNumber`))
      ;[1 0 0.3047] Checks if the boat's spawner id matches this spawner's id
      (for _array_element_2 (`self.Spawners`)
        (if (== (`local.CurrentSpawnerID`) (`/Game/Blueprints/Core/Boats/BP_BoatSpawner.SpawnerID` _array_element_2))
          (bind _boat_2 (`/Game/Blueprints/Core/Boats/BP_BoatSpawner.SpawnBoat` _array_element_2 (`local.CurrentBoatType`)))
          (bind _asaic_boat (cast `/Game/Blueprints/Core/Boats/AIC_Boat` (`AIBlueprintHelperLibrary.GetAIController` _boat_2)))
          (`/Game/Blueprints/Core/Boats/AIC_Boat.MoveBoat` _asaic_boat (`local.CurrentBoatDestination`) _boat_2))))))

(fn `UserConstructionScript`)