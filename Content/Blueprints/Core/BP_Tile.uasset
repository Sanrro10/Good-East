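; Grid tile for the defense game that registers with GM_DefenseGame, tracks commander occupancy and overlapping ally or enemy units, and can spawn boats.
; The construction script sets height, type sprite and tag, assigns unique spawner IDs, and builds houses.
; Houses merge linked secondary tiles, centering a child actor sized by tile count.
; Certain tile types bind to game-mode show/hide events, displaying a grid material that reflects occupancy.
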(event `ShowTiles`
  (bind _grid (`self.Grid`))
  (if (`self.bIsOcupied`)
    (`PrimitiveComponent.SetMaterial` _grid 0 "/Game/Art/Materials/M_Grid.M_Grid")
    (else
      (`PrimitiveComponent.SetMaterial` _grid 0 "/Game/Art/Materials/MI_GridWhite.MI_GridWhite")))
  (`SceneComponent.SetVisibility` (`self.Grid`) true true))

(event `self.ReceiveBeginPlay`
  (bind _asgm_defense_game (cast `/Game/Blueprints/Core/GM_DefenseGame` (`GameplayStatics.GetGameMode`)))
  (set `self.GM Defense Game` _asgm_defense_game)
  (`SceneComponent.SetVisibility` (`self.Grid`) false true)
  (`/Game/Blueprints/Core/GM_DefenseGame.Add Tile` (`self.GM Defense Game`) self)
  (if (or (`|EnumEquality` (`self.Type`) "NewEnumerator0") (`|EnumEquality` (`self.Type`) "NewEnumerator3"))
    (bind _asgm_defense_game_2 (cast `/Game/Blueprints/Core/GM_DefenseGame` (`GameplayStatics.GetGameMode`)))
    (add `/Game/Blueprints/Core/GM_DefenseGame.ShowTiles` _asgm_defense_game_2 (delegate `ShowTiles`))
    (add `/Game/Blueprints/Core/GM_DefenseGame.HideTiles` _asgm_defense_game_2 (delegate `HideTiles`))))

(event `HideTiles`
  (`SceneComponent.SetVisibility` (`self.Grid`) false true))

(event `self.Box.OnComponentBeginOverlap`
  (params (OverlappedComponent :type "PrimitiveComponent Object Reference") (OtherActor :type "Actor Object Reference") (OtherComp :type "PrimitiveComponent Object Reference") (OtherBodyIndex :type Integer) (bFromSweep :type Boolean) (SweepResult :type "HitResult Structure (by ref)"))
  (bind _asbp_unit (cast `/Game/Blueprints/Core/Units/BP_Unit` OtherActor))
  (if (`|EnumInequality` (`/Game/Blueprints/Core/Units/BP_Unit.GetCurrentState` _asbp_unit) "NewEnumerator5")
    (`self.Add  Current Unit` _asbp_unit)))

(event `self.Box.OnComponentEndOverlap`
  (params (OverlappedComponent :type "PrimitiveComponent Object Reference") (OtherActor :type "Actor Object Reference") (OtherComp :type "PrimitiveComponent Object Reference") (OtherBodyIndex :type Integer))
  (bind _asbp_unit (cast `/Game/Blueprints/Core/Units/BP_Unit` OtherActor))
  (`self.Remove Current Unit` _asbp_unit))

(fn `Add  Current Unit`
  (params (Unit :type "/Game/Blueprints/Core/Units/BP_Unit Object Reference"))
  (set `/Game/Blueprints/Core/Units/BP_Unit.Current Tile` self Unit)
  (if (`/Game/Blueprints/Core/Units/BP_Unit.isEnemy` Unit)
    (`KismetArrayLibrary.Array_AddUnique` (`self.EnemiesCurrentlyOnTile`) Unit)
    (`KismetSystemLibrary.PrintString` (`KismetStringLibrary.Concat_StrStr` "ENEMY ADDED: " (`KismetSystemLibrary.GetDisplayName` Unit)) true true (struct :`R` 1.0 :`B` 0.039114 :`A` 1.0) 20.0)
    (else
      (`KismetArrayLibrary.Array_AddUnique` (`self.AlliesCurrentlyOnTile`) Unit)
      (`KismetSystemLibrary.PrintString` (`KismetStringLibrary.Concat_StrStr` "ALLY ADDED: " (`KismetSystemLibrary.GetDisplayName` Unit)) true true (struct :`G` 1.0 :`B` 0.016063 :`A` 1.0) 20.0))))

(fn `Get Adjacent Tiles`
  (params (Range :type Integer))
  (returns (`Adjacent Tiles` :type "Array of /Game/Blueprints/Core/BP_Tile Object Reference"))
  (bind _adjacent_tiles (`/Game/Blueprints/Core/GM_DefenseGame.Get Adjacent Tiles` (`self.GM Defense Game`) Range (`self.Tile Index`)))
  (return _adjacent_tiles))

(fn `GetCenterLocation`
  (returns (Location :type "Vector Structure"))
  (return (`SceneComponent.K2_GetComponentLocation` (`self.Center`))))

(fn `InitializeHouse`
  (locals (HousePosition :type "Vector Structure") (LocalSecondaryHouseTiles :type "Array of /Game/Blueprints/Core/BP_Tile Object Reference"))
  (bind _localsecondaryhousetiles (`local.LocalSecondaryHouseTiles`))
  (for _array_element (`self.SecondaryHouseTilesArray`)
    (`/Engine/EditorBlueprintResources/StandardMacros.IsValid` _array_element
      (:`Is Valid`
        (`KismetArrayLibrary.Array_AddUnique` (`local.LocalSecondaryHouseTiles`) _array_element)
        (`KismetArrayLibrary.Array_RemoveItem` (`self.PreviousSecondaryHouseTilesArray`) _array_element))))
  (for _array_element_2 (`self.PreviousSecondaryHouseTilesArray`)
    (`self.SetTileType` _array_element_2 "NewEnumerator0")
    (`KismetArrayLibrary.Array_Clear` (`/Game/Blueprints/Core/BP_Tile.SecondaryHouseTilesArray` _array_element_2)))
  (if (`KismetArrayLibrary.Array_IsEmpty` (`local.LocalSecondaryHouseTiles`))
    (`self.SpawnHouse` 0)
    (`KismetArrayLibrary.Array_Clear` (`self.PreviousSecondaryHouseTilesArray`))
    (else
      (set `local.HousePosition` (`self.GetCenterLocation`))
      (for _array_element_3 _localsecondaryhousetiles
        (`self.SetTileType` _array_element_3 "NewEnumerator6")
        (bind _secondaryhousetilesarray (`/Game/Blueprints/Core/BP_Tile.SecondaryHouseTilesArray` _array_element_3))
        (`KismetArrayLibrary.Array_Clear` _secondaryhousetilesarray)
        (`KismetArrayLibrary.Array_Add` _secondaryhousetilesarray self)
        (set `local.HousePosition` (+ (`local.HousePosition`) (`self.GetCenterLocation` _array_element_3))))
      (`SceneComponent.K2_SetWorldLocation` (`self.ChildActor`) (/ (`local.HousePosition`) (+ (`KismetArrayLibrary.Array_Length` _localsecondaryhousetiles) 1)) false false)
      (`self.SpawnHouse` (`KismetArrayLibrary.Array_Length` (`local.LocalSecondaryHouseTiles`)))
      (set `self.PreviousSecondaryHouseTilesArray` (`local.LocalSecondaryHouseTiles`)))))

(fn `Remove Current Unit`
  (params (Unit :type "/Game/Blueprints/Core/Units/BP_Unit Object Reference"))
  (if (`/Game/Blueprints/Core/Units/BP_Unit.isEnemy` Unit)
    (`KismetArrayLibrary.Array_RemoveItem` (`self.EnemiesCurrentlyOnTile`) Unit)
    (else
      (`KismetArrayLibrary.Array_RemoveItem` (`self.AlliesCurrentlyOnTile`) Unit))))

(fn `Set Spawner ID`
  (params (`Spawner Array` :type "Array of /Game/Blueprints/Core/BP_Tile Object Reference"))
  (locals (`Current ID Array` :type "Array of Integer"))
  (for _array_element `Spawner Array`
    (if (!= _array_element self)
      (`KismetArrayLibrary.Array_AddUnique` (`local.Current ID Array`) (`/Game/Blueprints/Core/BP_Tile.Spawner ID` _array_element))))
  (for _index (range 17)
    (if (not (`KismetArrayLibrary.Array_Contains` (`local.Current ID Array`) _index))
      (set `self.Spawner ID` _index)
      (break))))

(fn `SetCommander`
  (params (Commander :type "/Game/Blueprints/Core/Units/Commander/BP_Commander Object Reference"))
  (`/Engine/EditorBlueprintResources/StandardMacros.IsValid` Commander
    (:`Is Valid`
      (set `self.Commander` Commander)
      (set `self.bIsOcupied` true))
    (:`Is Not Valid`
      (set `self.Commander` null)
      (set `self.bIsOcupied` false))))

(fn `SetTileType`
  (params (Type :type "/Game/Structures+Enumerators/ETileTypes Enum" :default "NewEnumerator0"))
  (bind _type (`self.Type`))
  (bind (_value _returnvalue) (`BlueprintMapLibrary.Map_Find` (`self.TileTypesSpritesMap`) (`self.Type`)))
  (set `self.Type` Type)
  (`|ExecutionSequence`
    (:`then_0`
      (if _returnvalue
        (`BillboardComponent.SetSprite` (`self.Center`) _value)))
    (:`then_1`
      (if (and (`|EnumInequality` _type "NewEnumerator6") (`|EnumInequality` _type "NewEnumerator5"))
        (`KismetArrayLibrary.Array_Clear` (`self.SecondaryHouseTilesArray`))
        (`KismetArrayLibrary.Array_Clear` (`self.PreviousSecondaryHouseTilesArray`))
        (set `self.House` null)))))

(fn `SpawnBoat`
  (params (`Boat Type` :type "/Game/Structures+Enumerators/EBoatType Enum" :default "NewEnumerator0"))
  (returns (Boat :type "/Game/Blueprints/Core/Boats/BP_Boat Object Reference"))
  (locals (BoatToSpawn :type "Actor Class Reference"))
  (switch `/Game/Structures+Enumerators/EBoatType` `Boat Type`
    (:`NewEnumerator0`
      (set `local.BoatToSpawn` "/Game/Blueprints/Core/Boats/BP_Boat_Basic.BP_Boat_Basic_C"))
    (:`NewEnumerator1`
      (set `local.BoatToSpawn` "/Game/Blueprints/Core/Boats/BP_Boat_Big.BP_Boat_Big_C")))
  (bind _returnvalue (`|SpawnActorFromClass` (`local.BoatToSpawn`) (`self.GetTransform`) "AdjustIfPossibleButAlwaysSpawn" "MultiplyWithRoot" null null))
  (bind _asbp_boat (cast `/Game/Blueprints/Core/Boats/BP_Boat` _returnvalue))
  (return _asbp_boat))

(fn `SpawnHouse`
  (params (HouseTileNumber :type Integer))
  (locals (HouseSize :type "Actor Class Reference"))
  (bind _childactor (`self.ChildActor`))
  (`|ExecutionSequence`
    (:`then_0`
      (if (== HouseTileNumber 0)
        (set `local.HouseSize` "/Game/Blueprints/Core/Houses/BP_HouseSmall.BP_HouseSmall_C")
        (elif (== HouseTileNumber 1)
          (set `local.HouseSize` "/Game/Blueprints/Core/Houses/BP_HouseMedium.BP_HouseMedium_C")
          (elif (== HouseTileNumber 3)
            (set `local.HouseSize` "/Game/Blueprints/Core/Houses/BP_HouseBig.BP_HouseBig_C")))))
    (:`then_1`
      (`ChildActorComponent.SetChildActorClass` _childactor (`local.HouseSize`))
      (bind _asbp_house (cast `/Game/Blueprints/Core/Houses/BP_House` (`ChildActorComponent.ChildActor` _childactor)))
      (bind _output_get (set `self.House` _asbp_house))
      (set `/Game/Blueprints/Core/Houses/BP_House.House Tile` self _output_get)
      (`/Game/Blueprints/Core/Houses/BP_House.ChangeHouseType` _output_get (`self.HouseType`)))))

(fn `UserConstructionScript`
  (bind (_returnvalue_x _returnvalue_y) (`KismetMathLibrary.BreakVector` (`self.K2_GetActorLocation`)))
  (bind (_value _returnvalue) (`BlueprintMapLibrary.Map_Find` (`self.TileTypesSpritesMap`) (`self.Type`)))
  (`self.K2_SetActorLocation` (`KismetMathLibrary.MakeVector` _returnvalue_x _returnvalue_y (* (`self.Height`) 400.0)) false true)
  (if _returnvalue
    (`BillboardComponent.SetSprite` (`self.Center`) _value)
    ;[0.03125 1 0] House
    (if (`|EnumEquality` "NewEnumerator5" (`self.Type`))
      (`self.InitializeHouse`))
    (set `self.Tags` (`|MakeArray` (`|GetEnumeratorName` (`self.Type`))))
    (if (`|EnumEquality` (`self.Type`) "NewEnumerator3")
      (bind _outactors (`GameplayStatics.GetAllActorsOfClassWithTag` "BP_Tile_C" (`|GetEnumeratorName` (`self.Type`))))
      (`self.Set Spawner ID` _outactors)
      (elif (`|EnumEquality` (`self.Type`) "NewEnumerator4")
        (bind _outactors_2 (`GameplayStatics.GetAllActorsOfClassWithTag` "BP_Tile_C" (`|GetEnumeratorName` (`self.Type`))))
        (`self.Set Spawner ID` _outactors_2)))))