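; BP_Archer is an archer unit that fires homing arrows at a target unit with a chance to miss.
; SpawnArrow creates a BP_Arrow at the archer's transform, stores it as ShotArrow and prints its name.
; ShootArrow rolls against HitChance, homing the arrow on the target's capsule or on FailTarget, teleported randomly near the target, then sets its speed.
; The event graph holds only disabled stubs, so neither function is called here.
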(fn `ShootArrow`
  (locals (ArrowProjectileComponent :type "ProjectileMovementComponent Object Reference"))
  (bind _arrowprojectilecomponent (`local.ArrowProjectileComponent`))
  (set `local.ArrowProjectileComponent` (`/Game/Blueprints/Core/Projectile/BP_Arrow.ProjectileMovement` (`self.ShotArrow`)))
  (if (< (`KismetMathLibrary.RandomFloatInRange` 0.0 1.0) (`self.HitChance`))
    (set `ProjectileMovementComponent.HomingTargetComponent` (`Character.CapsuleComponent` (`self.TargetUnit`)) (`local.ArrowProjectileComponent`))
    (else
      (`SceneComponent.K2_SetWorldLocation` (`self.FailTarget`) (`KismetMathLibrary.RandomPointInBoundingBox` (`self.K2_GetActorLocation` (`self.TargetUnit`)) (200.0 200.0 0.0)) false true)
      (set `ProjectileMovementComponent.HomingTargetComponent` (`self.FailTarget`) (`local.ArrowProjectileComponent`))))
  (set `ProjectileMovementComponent.InitialSpeed` 10.0 _arrowprojectilecomponent)
  (set `ProjectileMovementComponent.MaxSpeed` 10.0 _arrowprojectilecomponent))

(fn `SpawnArrow`
  (bind _returnvalue (`|SpawnActorFromClass` "/Game/Blueprints/Core/Projectile/BP_Arrow.BP_Arrow_C" (`self.GetTransform` self) "AdjustIfPossibleButAlwaysSpawn" "MultiplyWithRoot" self self))
  (bind _output_get (set `self.ShotArrow` _returnvalue))
  (`KismetSystemLibrary.PrintString` (`KismetSystemLibrary.GetDisplayName` _output_get)))

(fn `UserConstructionScript`
  (`parent.UserConstructionScript`))