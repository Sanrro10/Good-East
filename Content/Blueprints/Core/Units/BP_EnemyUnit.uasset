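; BP_EnemyUnit is an enemy unit that finds and burns houses.
; GetNearestHouse picks the house with the shortest navigation path using Ally_NavFilter.
; BurnHouse uses placeholder delays until an attack animation exists, firing dispatchers bound at BeginPlay that damage the target, make the unit interruptible and end the burning state.
; CreateTorch spawns and ignites a torch at the left-hand socket.
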(event `Burn House`
  (params (House :type "/Game/Blueprints/Core/Houses/BP_House Object Reference"))
  (set `self.Target House` House)
  (set `self.Burning House` true)
  ;[0.7812 1 0] Remove when making attack house animation
  (`KismetSystemLibrary.Delay` 1.0)
  (`self.House Burn Deal Damage`)
  (`KismetSystemLibrary.Delay` 0.5)
  (`self.Finish House Burn Animation`))

(event `self.ReceiveBeginPlay`
  (`parent.ReceiveBeginPlay`)
  (add `self.Finish House Burn Animation` (delegate `Finish House Attack Event`))
  (add `self.House Burn Deal Damage` (delegate `House Attack Deal Damage Event`)))

(event `Finish House Attack Event`
  (set `self.Burning House` false))

(event `House Attack Deal Damage Event`
  (`/Game/Blueprints/Core/Houses/BP_House.Receive Damage` (`self.Target House`))
  (set `self.CanBeInterrupted` true))

(event `CreateTorch`
  (bind _returnvalue (`|SpawnActorFromClass` "/Game/Blueprints/Core/Projectile/BP_Torch.BP_Torch_C" (`SceneComponent.GetSocketTransform` (`self.Mesh`) "HandL_Torch" "RTS_World") "AdjustIfPossibleButAlwaysSpawn" "MultiplyWithRoot" null null))
  ;[1 0.1641 0] We have to decide if we place a time between spawn an ignition
  (`/Game/Blueprints/Core/Projectile/BP_Torch.IgniteFire` _returnvalue))

(fn `Get Nearest House`
  (returns (`Nearest House` :type "/Game/Blueprints/Core/Houses/BP_House Object Reference"))
  (locals (`Current Path Distance` :type "Float (double-precision)" :default 1e+32) (CurrentHouse :type "/Game/Blueprints/Core/Houses/BP_House Object Reference") (NearestHouse :type "/Game/Blueprints/Core/Houses/BP_House Object Reference"))
  (for _array_element (`/Game/Blueprints/Core/GM_DefenseGame.Get Houses Array` (`self.GameMode`))
    (bind _output_get (set `local.CurrentHouse` _array_element))
    (bind _returnvalue (`NavigationSystemV1.FindPathToActorSynchronously` (`NavigationSystemV1.GetNavigationSystem`) (`self.K2_GetActorLocation`) _output_get 50.0 self "/Game/Blueprints/Core/Navigation/Ally_NavFilter.Ally_NavFilter_C"))
    (bind _returnvalue_2 (`NavigationPath.GetPathLength` _returnvalue))
    (if (< _returnvalue_2 (`local.Current Path Distance`))
      (set `local.Current Path Distance` _returnvalue_2)
      (set `local.NearestHouse` (`local.CurrentHouse`))))
  (return (`local.NearestHouse`)))

(fn `UserConstructionScript`
  (`parent.UserConstructionScript`))