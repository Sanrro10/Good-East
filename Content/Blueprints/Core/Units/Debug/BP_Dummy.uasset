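; BP_Dummy is a debug unit that serves as a dummy and visibly reacts when it takes damage.
; Its receive-damage event plays an interruption montage on its mesh.
; It has no other active logic: the default BeginPlay, overlap and Tick events are disabled, and the construction script only calls its parent.
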(event `self.Event Receive Damage`
  (params (Damage :type "Float (double-precision)") (KnockBackValue :type "Vector Structure"))
  (`|PlayMontage` (`self.Mesh`) (`self.Interruption Montage`)))

(fn `UserConstructionScript`
  (`parent.UserConstructionScript`))