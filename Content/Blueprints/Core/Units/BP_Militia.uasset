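; BP_Militia is a militia unit Blueprint that sets its facing after movement in relation to its Commander.
; UpdateRotationAfterMovement takes the unit's own desired rotation while the Commander moves, otherwise the Commander's.
; It resets the lerp alpha and restarts a fast looping SmoothRotation timer, whose function is not defined here.
; Event graph and construction script add no logic of their own.
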(fn `UpdateRotationAfterMovement`
  (bind _commander (`self.Commander`))
  (`KismetSystemLibrary.K2_ClearTimer` null "SmoothRotation")
  (set `self.LerpAlpha` 0.0)
  (if (`/Game/Blueprints/Core/Units/BP_Unit.Moving` _commander)
    (set `self.DesiredRotation` (`self.GetDesiredRotation`))
    (else
      (set `self.DesiredRotation` (`self.GetDesiredRotation` _commander))))
  (`KismetSystemLibrary.K2_SetTimer` null "SmoothRotation" 0.01 true))

(fn `UserConstructionScript`
  (`parent.UserConstructionScript`))