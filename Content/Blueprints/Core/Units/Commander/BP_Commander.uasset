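; Squad commander for a tile-based defense game that carries an odachi and colored flag and leads up to eight units of one class.
; Units map to formation points, rearranged by squad size, and share the commander's avoidance group.
; Tile orders propagate to every unit, with nav-path length choosing fallback tiles.
; House moves require missing units; healing respawns them on a timer, and damage reduces commander health only once none remain.
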(event `self.ReceiveBeginPlay`
  (`parent.ReceiveBeginPlay`)
  (`/Game/Blueprints/Core/GM_DefenseGame.Add Commander` (`self.GameMode`) self)
  (bind _returnvalue (`|SpawnActorFromClass` "/Game/Blueprints/Core/Weapons/BP_Odachi.BP_Odachi_C" (`SceneComponent.GetSocketTransform` (`self.Mesh`) "HandR_Odachi_Socket" "RTS_World") "Undefined" "MultiplyWithRoot" null null))
  (bind _output_get (set `self.Odachi` _returnvalue))
  (`self.K2_AttachToComponent` _output_get (`self.Mesh`) "HandR_Odachi_Socket" "SnapToTarget" "SnapToTarget" "SnapToTarget" false)
  (bind _returnvalue_2 (`|SpawnActorFromClass` "/Game/Blueprints/Core/Weapons/BP_Flag.BP_Flag_C" (`SceneComponent.GetSocketTransform` (`self.Mesh`) "Spine_01_Flag_Socket" "RTS_World") "Undefined" "MultiplyWithRoot" null null))
  (bind _output_get_2 (set `self.Flag` _returnvalue_2))
  (`self.K2_AttachToComponent` _output_get_2 (`self.Mesh`) "Spine_01_Flag_Socket" "SnapToTarget" "SnapToTarget" "SnapToTarget" false))

(event `Event Bind To Commander's Repositioning`
  (params (Commander :type "/Game/Blueprints/Core/Units/Commander/BP_Commander Object Reference"))
  (add `self.Repositioning Completed` Commander (delegate `Restore Formation Scale`)))

(event `Restore Formation Scale`
  (clear `self.Repositioning Completed`)
  (`KismetSystemLibrary.Delay` 0.2)
  (`SceneComponent.SetRelativeScale3D` (`self.FormationPositiosCenter`) (0.7 0.7 0.7))
  (`self.Move to Tile` (`self.Desired Tile`)))

(event `Heal Commander`
  (`self.SpawnUnit` (`self.GetEmptyFormationPosition`))
  (if (not (< (`BlueprintMapLibrary.Map_Length` (`self.UnitsArray`)) 8))
    (`KismetSystemLibrary.K2_ClearAndInvalidateTimerHandle` (stale `Start Healing Event` _returnvalue) :!label _label)))

(event `Start Healing Event`
  (params (`Heal Rate` :type "Float (double-precision)"))
  (if (< (`KismetArrayLibrary.Array_Length` (`self.GetUnitsArray`)) 8)
    (bind _returnvalue (`KismetSystemLibrary.K2_SetTimerDelegate` (delegate `Heal Commander`) `Heal Rate` true))
    (else
      (goto _label))))

(event `Receive Damage Event_1`
  (params (Damage :type "Float (double-precision)"))
  (if (`self.CanBeInterrupted`)
    (`self.Set State` "NewEnumerator4")
    (`|PlayMontage` (`self.Mesh`) (`self.Interruption Montage`)
      (:`then`
        (if (`BlueprintMapLibrary.Map_IsEmpty` (`self.UnitsArray`)) :!label _label_2
          (bind _output_get (set `self.HealthPoints` (- (`self.HealthPoints`) Damage)))
          (`KismetArrayLibrary.Array_Clear` (`self.EnemiesToIgnore`))
          (if (<= _output_get 0.0)
            (`self.Set State` "NewEnumerator5")
            (`self.Die Event`))))
      (:`OnCompleted`
        (`self.Set State` (`self.GetPreviousState`))))
    (else
      (goto _label_2))))

(fn `Get Can Heal`
  (returns (`Can Heal` :type Boolean))
  (return (< (`BlueprintMapLibrary.Map_Length` (`self.UnitsArray`)) 8)))

(fn `GetClosestTileInArray`
  (params (Tiles :type "Array of /Game/Blueprints/Core/BP_Tile Object Reference"))
  (returns (`Closest Tile` :type "/Game/Blueprints/Core/BP_Tile Object Reference"))
  (locals (`Current Path Distance` :type "Float (double-precision)") (MinDistance :type "Float (double-precision)" :default 1e+26) (`Current Tile` :type "/Game/Blueprints/Core/BP_Tile Object Reference") (`Closest Tile Var` :type "/Game/Blueprints/Core/BP_Tile Object Reference"))
  (for _array_element Tiles
    (set `local.Current Tile` _array_element)
    (bind _returnvalue (`NavigationSystemV1.FindPathToActorSynchronously` (`NavigationSystemV1.GetNavigationSystem`) (`self.K2_GetActorLocation`) (`local.Current Tile`) 50.0 self "/Game/Blueprints/Core/Navigation/Ally_NavFilter.Ally_NavFilter_C"))
    (bind _returnvalue_2 (`NavigationPath.GetPathLength` _returnvalue))
    (set `local.Current Path Distance` _returnvalue_2)
    (if (and (> _returnvalue_2 0.0) (< (`local.Current Path Distance`) (`local.MinDistance`)))
      (set `local.MinDistance` (`local.Current Path Distance`))
      (set `local.Closest Tile Var` (`local.Current Tile`))))
  (return (`local.Closest Tile Var`)))

(fn `GetEmptyFormationPosition`
  (returns (FormationPosition :type "SceneComponent Object Reference"))
  (for _array_element (`self.SpawnPositions`)
    (bind _values (`BlueprintMapLibrary.Map_Values` (`self.UnitsArray`)))
    (if (not (`KismetArrayLibrary.Array_Contains` _values _array_element))
      (return _array_element))))

(fn `GetUnitsArray`
  (returns (Units :type "Array of /Game/Blueprints/Core/Units/BP_AlliedUnit Object Reference"))
  (bind _keys (`BlueprintMapLibrary.Map_Keys` (`self.UnitsArray`)))
  (return _keys))

(fn `Initialize Commander`
  (locals (CurrentUnitDesiredPosition :type "Vector Structure" :default (0.0 0.0 0.0)))
  (`/Game/Blueprints/Core/Weapons/BP_Flag.SetColor` (`self.Flag`) (`self.Color`))
  (set `self.DesiredPosition` (`self.K2_GetActorLocation`))
  (set `/Game/Blueprints/Core/Units/Militia/BP_Militia.Commander` self)
  (set `self.Current Tile` (`self.Desired Tile`))
  (`self.Set Spawn Unit Class`)
  (bind (_avoidancegroup _groupstoavoid) (`self.Request Avoidance Groups ID`))
  (set `self.Avoidance Group Var` _avoidancegroup)
  (set `self.Groups To Avoid Var` _groupstoavoid)
  (`CharacterMovementComponent.SetAvoidanceGroupMask` (`self.CharacterMovement`) _avoidancegroup)
  (`CharacterMovementComponent.SetGroupsToAvoidMask` (`self.CharacterMovement`) _avoidancegroup)
  (bind _output_get (set `self.GroupsToIgnore Var` _avoidancegroup))
  (bind _structout (setmembers `NavAvoidanceMask` :`StructRef` _output_get :`bGroup25` true))
  (`CharacterMovementComponent.SetGroupsToIgnoreMask` (`self.CharacterMovement`) _structout)
  (for _array_element (`self.SpawnPositions`)
    (`self.SpawnUnit` _array_element)))

(fn `Look for Enemies Around Desired Tile`
  (returns (EnemiesAroundCurrentTile :type "Array of /Game/Blueprints/Core/Units/BP_Unit Object Reference"))
  (locals (EnemiesAroundCurrentTileArray :type "Array of /Game/Blueprints/Core/Units/BP_Unit Object Reference"))
  (bind _adjacent_tiles (`/Game/Blueprints/Core/BP_Tile.Get Adjacent Tiles` (`self.Desired Tile`) (`self.Get Current Range`)))
  (if (`self.isEnemy`)
    (for _array_element _adjacent_tiles
      (for _array_element_2 (`/Game/Blueprints/Core/BP_Tile.AlliesCurrentlyOnTile` _array_element)
        (`KismetArrayLibrary.Array_AddUnique` (`local.EnemiesAroundCurrentTileArray`) _array_element_2)))
    (else
      (for _array_element_3 _adjacent_tiles
        (for _array_element_4 (`/Game/Blueprints/Core/BP_Tile.EnemiesCurrentlyOnTile` _array_element_3)
          (`KismetArrayLibrary.Array_AddUnique` (`local.EnemiesAroundCurrentTileArray`) _array_element_4)))))
  (return (`local.EnemiesAroundCurrentTileArray`)))

(fn `Move To House`
  (params (`House Tile` :type "/Game/Blueprints/Core/BP_Tile Object Reference"))
  (returns (Sucess :type Boolean))
  (bind _house (`/Game/Blueprints/Core/BP_Tile.GetHouse` `House Tile`))
  (if (`self.Get Can Heal`)
    (`/Engine/EditorBlueprintResources/StandardMacros.IsValid` _house
      (:`Is Valid`
        (`self.Update Desired Tile` `House Tile`)
        (set `self.DesiredPosition` (`/Game/Blueprints/Core/Houses/BP_House.GetDoorPosition` _house))
        (for _array_element (`self.GetUnitsArray`)
          (set `/Game/Blueprints/Core/Units/BP_Unit.DesiredPosition` (`self.DesiredPosition`) _array_element)
          (set `/Game/Blueprints/Core/Units/BP_AlliedUnit.HasRepositionOrder` true _array_element)
          (set `/Game/Blueprints/Core/Units/BP_Unit.Desired Tile` (`self.Desired Tile`) _array_element))
        (return true))
      (:`Is Not Valid`
        (`KismetSystemLibrary.PrintString` "HOUSE NOT VALID (Commander Move To House)")
        (return false)))
    (else
      (return false))))

(fn `Move to Tile`
  (params (Tile :type "/Game/Blueprints/Core/BP_Tile Object Reference"))
  (returns (Sucess :type Boolean))
  (locals (TileCenterLocation :type "Vector Structure" :default (0.0 0.0 0.0)))
  (if (`|EnumEquality` "NewEnumerator5" (`/Game/Blueprints/Core/BP_Tile.Type` Tile))
    (bind _sucess (`self.Move To House` Tile))
    (return _sucess)
    (elif (`|EnumEquality` (`/Game/Blueprints/Core/BP_Tile.Type` Tile) "NewEnumerator6")
      (bind _sucess_2 (`self.Move To House` (`|GetArrayItem` (`/Game/Blueprints/Core/BP_Tile.SecondaryHouseTilesArray` Tile))))
      (return _sucess_2)
      (else
        (`self.Update Desired Tile` Tile)
        (bind _output_get (set `local.TileCenterLocation` (`/Game/Blueprints/Core/BP_Tile.GetCenterLocation` Tile)))
        (set `self.DesiredPosition` _output_get)
        (for _array_element (`self.GetUnitsArray`)
          (set `/Game/Blueprints/Core/Units/BP_Unit.DesiredPosition` (+ (* (`SceneComponent.RelativeLocation` (`/Game/Blueprints/Core/Units/Militia/BP_Militia.FormationPosition` _array_element)) (`SceneComponent.RelativeScale3D` (`self.FormationPositiosCenter`))) (`local.TileCenterLocation`)) _array_element)
          (set `/Game/Blueprints/Core/Units/BP_AlliedUnit.HasRepositionOrder` true _array_element)
          (set `/Game/Blueprints/Core/Units/BP_Unit.Desired Tile` (`self.Desired Tile`) _array_element))
        (return true)))))

(fn `RemoveUnitFromCommander`
  (params (Unit :type "/Game/Blueprints/Core/Units/BP_AlliedUnit Object Reference (by ref)"))
  (`BlueprintMapLibrary.Map_Remove` (`self.UnitsArray`) Unit))

(fn `RepositionToAdjacentTile`
  (params (`Other Commander's Tile` :type "/Game/Blueprints/Core/BP_Tile Object Reference") (`Other Commander` :type "/Game/Blueprints/Core/Units/Commander/BP_Commander Object Reference"))
  (locals (`Other Tile` :type "/Game/Blueprints/Core/BP_Tile Object Reference") (AdjacentTiles :type "Array of /Game/Blueprints/Core/BP_Tile Object Reference") (`Range Var` :type Integer :default 1) (`Other Commander Var` :type "/Game/Blueprints/Core/Units/Commander/BP_Commander Object Reference"))
  (bind _closest_tile (`self.GetClosestTileInArray` (`local.AdjacentTiles`)))
  (set `local.Other Tile` `Other Commander's Tile`)
  (`self.Event Bind To Commander's Repositioning` `Other Commander`)
  (`SceneComponent.SetRelativeScale3D` (`self.FormationPositiosCenter`) (1.0 1.0 1.0))
  (bind _adjacent_tiles (`/Game/Blueprints/Core/BP_Tile.Get Adjacent Land Tiles` (`self.Current Tile`) (`local.Range Var`) :!label _label))
  (bind _output_get (set `local.AdjacentTiles` _adjacent_tiles))
  (if (`KismetArrayLibrary.Array_Contains` _output_get (`local.Other Tile`))
    (`self.Move to Tile` (`local.Other Tile`))
    (else
      (for _array_element (`/Game/Blueprints/Core/GM_DefenseGame.GetDesiredTiles` (`self.GameMode`))
        (`KismetArrayLibrary.Array_RemoveItem` (`local.AdjacentTiles`) _array_element))
      (`/Engine/EditorBlueprintResources/StandardMacros.IsValid` _closest_tile
        (:`Is Valid`
          (`self.Move to Tile` _closest_tile))
        (:`Is Not Valid`
          (`/Engine/EditorBlueprintResources/StandardMacros.IncrementInt` (`local.Range Var`)
            (:`  `
              (goto _label))))))))

(fn `RepositionUnits`
  (`|ExecutionSequence`
    (:`then_0`
      (switch `int` (`BlueprintMapLibrary.Map_Length` (`self.UnitsArray`))
        (:`1`
          (`self.SetUnitPositionByIndex` 0 (`self.FormationPosition 2`)))
        (:`2`
          (`self.SetUnitPositionByIndex` 0 (`self.FormationPosition 1,5`))
          (`self.SetUnitPositionByIndex` 1 (`self.FormationPosition 2,5`)))
        (:`3`
          (`self.SetUnitPositionByIndex` 0 (`self.FormationPosition 1,5`))
          (`self.SetUnitPositionByIndex` 1 (`self.FormationPosition 2,5`))
          (`self.SetUnitPositionByIndex` 2 (`self.FormationPosition 8`)))
        (:`4`
          (`self.SetUnitPositionByIndex` 0 (`self.FormationPosition 1,5`))
          (`self.SetUnitPositionByIndex` 1 (`self.FormationPosition 2,5`))
          (`self.SetUnitPositionByIndex` 2 (`self.FormationPosition 7,5`))
          (`self.SetUnitPositionByIndex` 3 (`self.FormationPosition 8,5`)))
        (:`5`
          (`self.SetUnitPositionByIndex` 0 (`self.FormationPosition 1,5`))
          (`self.SetUnitPositionByIndex` 1 (`self.FormationPosition 2,5`))
          (`self.SetUnitPositionByIndex` 2 (`self.FormationPosition 4`))
          (`self.SetUnitPositionByIndex` 3 (`self.FormationPosition 6`))
          (`self.SetUnitPositionByIndex` 4 (`self.FormationPosition 8`)))
        (:`6`
          (`self.SetUnitPositionByIndex` 0 (`self.FormationPosition 1,5`))
          (`self.SetUnitPositionByIndex` 1 (`self.FormationPosition 2,5`))
          (`self.SetUnitPositionByIndex` 2 (`self.FormationPosition 4`))
          (`self.SetUnitPositionByIndex` 3 (`self.FormationPosition 6`))
          (`self.SetUnitPositionByIndex` 4 (`self.FormationPosition 7,5`))
          (`self.SetUnitPositionByIndex` 5 (`self.FormationPosition 8,5`)))
        (:`7`
          (`self.SetUnitPositionByIndex` 0 (`self.FormationPosition 1`))
          (`self.SetUnitPositionByIndex` 1 (`self.FormationPosition 2`))
          (`self.SetUnitPositionByIndex` 2 (`self.FormationPosition 3`))
          (`self.SetUnitPositionByIndex` 3 (`self.FormationPosition 4`))
          (`self.SetUnitPositionByIndex` 4 (`self.FormationPosition 6`))
          (`self.SetUnitPositionByIndex` 5 (`self.FormationPosition 7,5`))
          (`self.SetUnitPositionByIndex` 6 (`self.FormationPosition 8,5`)))
        (:`8`
          (`self.SetUnitPositionByIndex` 0 (`self.FormationPosition 1`))
          (`self.SetUnitPositionByIndex` 1 (`self.FormationPosition 2`))
          (`self.SetUnitPositionByIndex` 2 (`self.FormationPosition 3`))
          (`self.SetUnitPositionByIndex` 3 (`self.FormationPosition 4`))
          (`self.SetUnitPositionByIndex` 4 (`self.FormationPosition 6`))
          (`self.SetUnitPositionByIndex` 5 (`self.FormationPosition 7`))
          (`self.SetUnitPositionByIndex` 6 (`self.FormationPosition 8`))
          (`self.SetUnitPositionByIndex` 7 (`self.FormationPosition 9`)))))
    (:`then_1`
      (`self.Move to Tile` (`self.Desired Tile`)))))

(fn `Request Avoidance Groups ID`
  (returns (AvoidanceGroup :type "NavAvoidanceMask Structure") (GroupsToAvoid :type "NavAvoidanceMask Structure"))
  (bind _asgm_defense_game (cast `/Game/Blueprints/Core/GM_DefenseGame` (`GameplayStatics.GetGameMode`)))
  (bind (_avoidancegroup _groupstoavoid) (`/Game/Blueprints/Core/GM_DefenseGame.Get Avoidance Group ID` _asgm_defense_game))
  (return _avoidancegroup _groupstoavoid))

(fn `Set Spawn Unit Class`
  (if (`|EnumEquality` (`self.UnitType`) "NewEnumerator0")
    (set `self.UnitClass` "/Game/Blueprints/Core/Units/Militia/BP_Militia.BP_Militia_C")
    (elif (or (`|EnumEquality` (`self.UnitType`) "NewEnumerator1") (`|EnumEquality` (`self.UnitType`) "NewEnumerator2") (`|EnumEquality` (`self.UnitType`) "NewEnumerator3"))
      (set `self.UnitClass` "/Game/Blueprints/Core/Units/Monk/BP_Monk.BP_Monk_C")
      (elif (or (`|EnumEquality` (`self.UnitType`) "NewEnumerator4") (`|EnumEquality` (`self.UnitType`) "NewEnumerator5") (`|EnumEquality` (`self.UnitType`) "NewEnumerator6"))
        (set `self.UnitClass` "/Game/Blueprints/Core/Units/Pikeman/BP_Pikeman.BP_Pikeman_C")
        (else
          (set `self.UnitClass` "/Game/Blueprints/Core/Units/Archer/BP_Archer.BP_Archer_C"))))))

(fn `SetUnitPositionByIndex`
  (params (Index :type Integer) (`Formation Position` :type "SceneComponent Object Reference"))
  (bind _units (`self.GetUnitsArray`))
  (bind _output (`|GetArrayItem` _units Index))
  (if (`KismetArrayLibrary.Array_IsValidIndex` _units Index)
    (set `/Game/Blueprints/Core/Units/BP_Unit.FormationPosition` `Formation Position` _output)
    (`BlueprintMapLibrary.Map_Add` (`self.UnitsArray`) _output `Formation Position`)
    (else
      (`KismetSystemLibrary.PrintString` "INDEX NOT VALID"))))

(fn `SpawnUnit`
  (params (FormationPosition :type "SceneComponent Object Reference"))
  (locals (CurrentUnitDesiredPosition :type "Vector Structure"))
  (bind _returnvalue (`SceneComponent.K2_GetComponentLocation` FormationPosition))
  (set `local.CurrentUnitDesiredPosition` _returnvalue)
  (bind _returnvalue_2 (`|SpawnActorFromClass` (`self.UnitClass`) (`KismetMathLibrary.MakeTransform` _returnvalue (`self.K2_GetActorRotation`)) "AdjustIfPossibleButAlwaysSpawn" "MultiplyWithRoot" self self))
  (set `/Game/Blueprints/Core/Units/BP_Unit.isEnemy` (`self.isEnemy`) _returnvalue_2)
  (set `/Game/Blueprints/Core/Units/BP_Unit.Current Tile` (`self.Current Tile`) _returnvalue_2)
  (`BlueprintMapLibrary.Map_Add` (`self.UnitsArray`) _returnvalue_2 FormationPosition)
  (set `/Game/Blueprints/Core/Units/Militia/BP_Militia.FormationPosition` FormationPosition _returnvalue_2)
  (set `/Game/Blueprints/Core/Units/BP_AlliedUnit.Commander` self _returnvalue_2)
  (`self.Update Avoidance` _returnvalue_2 (`self.Avoidance Group Var`) (`self.Groups To Avoid Var`) (`self.GroupsToIgnore Var`))
  (set `/Game/Blueprints/Core/Units/BP_Unit.DesiredPosition` (`local.CurrentUnitDesiredPosition`) _returnvalue_2)
  (set `/Game/Blueprints/Core/Units/BP_Unit.Desired Tile` (`self.Desired Tile`) _returnvalue_2))

(fn `Update Desired Tile`
  (params (NewTile :type "/Game/Blueprints/Core/BP_Tile Object Reference"))
  (bind _desired_tile (`self.Desired Tile`))
  (`/Engine/EditorBlueprintResources/StandardMacros.IsValid` _desired_tile
    (:`Is Valid`
      (`/Game/Blueprints/Core/BP_Tile.SetCommander` _desired_tile null))
    (:`Is Not Valid`
      _))
  (bind _output_get (set `self.Desired Tile` NewTile))
  (`/Game/Blueprints/Core/BP_Tile.SetCommander` _output_get self)
  (set `self.HasRepositionOrder` true))

(fn `UpdateRotationAfterMovement`
  (set `self.DesiredRotation` (`self.GetDesiredRotation`))
  (set `self.LerpAlpha` 0.0)
  (`KismetSystemLibrary.K2_ClearTimer` null "SmoothRotation")
  (`KismetSystemLibrary.K2_SetTimer` null "SmoothRotation" 0.01 true)
  (for _array_element (`self.GetUnitsArray`)
    (`/Engine/EditorBlueprintResources/StandardMacros.IsValid` _array_element
      (:`Is Valid`
        (if (`/Game/Blueprints/Core/Units/BP_Unit.Moving` _array_element)
          _
          (elif (not (== (`self.GetDesiredRotation`) (`self.DesiredRotation`) :`ErrorTolerance` 5.0))
            (set `/Game/Blueprints/Core/Units/BP_AlliedUnit.DesiredRotation` (`self.DesiredRotation`) _array_element)
            (set `/Game/Blueprints/Core/Units/BP_AlliedUnit.LerpAlpha` 0.0 _array_element)
            (`KismetSystemLibrary.K2_ClearTimer` _array_element "SmoothRotation")
            (`KismetSystemLibrary.K2_SetTimer` _array_element "SmoothRotation" 0.01 true)))))))

(fn `UserConstructionScript`
  (`parent.UserConstructionScript`)
  (`KismetArrayLibrary.Array_Add` (`self.SpawnPositions`) (`self.FormationPosition 1`))
  (`KismetArrayLibrary.Array_Add` (`self.SpawnPositions`) (`self.FormationPosition 2`))
  (`KismetArrayLibrary.Array_Add` (`self.SpawnPositions`) (`self.FormationPosition 3`))
  (`KismetArrayLibrary.Array_Add` (`self.SpawnPositions`) (`self.FormationPosition 4`))
  (`KismetArrayLibrary.Array_Add` (`self.SpawnPositions`) (`self.FormationPosition 6`))
  (`KismetArrayLibrary.Array_Add` (`self.SpawnPositions`) (`self.FormationPosition 7`))
  (`KismetArrayLibrary.Array_Add` (`self.SpawnPositions`) (`self.FormationPosition 8`))
  (`KismetArrayLibrary.Array_Add` (`self.SpawnPositions`) (`self.FormationPosition 9`)))