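; Archer unit that spawns a bow in its hand and attacks a target unit with arrows.
; AttackUnit plays a montage whose notifies spawn an arrow in hand, then fire it, and calls OnFinishAttack on blend out.
; A hit-chance roll either makes the arrow home on the target or lobs it in an arc toward a random nearby point.
; Attack range grows with the current tile's height.
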(event `self.ReceiveBeginPlay`
  (`parent.ReceiveBeginPlay`)
  (bind _returnvalue (`|SpawnActorFromClass` "/Game/Blueprints/Core/Weapons/BP_Bow.BP_Bow_C" (`SceneComponent.GetSocketTransform` (`self.Mesh`) "HandWeaponSocket" "RTS_World") "Undefined" "MultiplyWithRoot" null null))
  (bind _output_get (set `self.Weapon` _returnvalue))
  (`self.K2_AttachToComponent` _output_get (`self.Mesh`) "HandWeaponSocket" "SnapToTarget" "SnapToTarget" "SnapToTarget" false))

(event `self.Attack Unit`
  (params (`Target Unit` :type "/Game/Blueprints/Core/Units/BP_Unit Object Reference"))
  (set `self.Attack Target Unit` `Target Unit`)
  (set `self.Attacking` true)
  (bind _notifyname (`|PlayMontage` (`self.Mesh`) (`self.Attack Montage`) (`self.Attack Play Rate`))
    (:`OnBlendOut`
      (set `self.Attacking` false)
      (`self.OnFinishAttack`))
    (:`OnNotifyBegin`
      (if (== _notifyname "Draw Arrow")
        (`self.Draw Arrow`)
        (else
          (`self.Shoot Arrow`))))))

(fn `Draw Arrow`
  (bind _returnvalue (`|SpawnActorFromClass` "/Game/Blueprints/Core/Projectile/BP_Arrow.BP_Arrow_C" (`SceneComponent.GetSocketTransform` (`self.Mesh`) "HandTorchSocket" "RTS_World") "AdjustIfPossibleButAlwaysSpawn" "MultiplyWithRoot" self self))
  (bind _output_get (set `self.Current Arrow` _returnvalue))
  (`/Engine/EditorBlueprintResources/StandardMacros.IsValid` _output_get
    (:`Is Valid`
      (`self.K2_AttachToComponent` _output_get (`self.Mesh`) "HandTorchSocket" "SnapToTarget" "SnapToTarget" "SnapToTarget" false))))

(fn `Get Current Range`
  (returns (Range :type Integer))
  (return (+ (`self.Range`) (`/Game/Blueprints/Core/BP_Tile.Height` (`self.Current Tile`)))))

(fn `GetCurrentRangeInDistance`
  (returns (AttackRangeInDistance :type "Float (double-precision)"))
  (return (* (`self.Get Current Range`) 400)))

(fn `Shoot Arrow`
  (bind _current_arrow (`self.Current Arrow`))
  (bind _projectilemovement (`/Game/Blueprints/Core/Projectile/BP_Arrow.ProjectileMovement` (`self.Current Arrow`)))
  (`|ExecutionSequence`
    (:`then_0`
      (if (< (`KismetMathLibrary.RandomFloatInRange` 0.0 1.0) (`self.HitChance`))
        (set `ProjectileMovementComponent.HomingTargetComponent` (`Character.CapsuleComponent` (`self.Attack Target Unit`)) (`/Game/Blueprints/Core/Projectile/BP_Arrow.ProjectileMovement` (`self.Current Arrow`)))
        (else
          (bind _outlaunchvelocity (`GameplayStatics.SuggestProjectileVelocity_CustomArc` (`self.K2_GetActorLocation` (`self.Current Arrow`)) (`KismetMathLibrary.RandomPointInBoundingBox` (`self.K2_GetActorLocation` (`self.Attack Target Unit`)) (200.0 200.0 0.0))))
          (`ProjectileMovementComponent.SetVelocityInLocalSpace` _projectilemovement _outlaunchvelocity)
          (set `ProjectileMovementComponent.bInitialVelocityInLocalSpace` true _projectilemovement))))
    (:`then_1`
      (set `/Game/Blueprints/Core/Projectile/BP_Arrow.Damage` (`self.Attack Damage`) _current_arrow)
      (set `/Game/Blueprints/Core/Projectile/BP_Arrow.Knock Back Strength` (`self.KnockBackStrength`) _current_arrow)
      (set `/Game/Blueprints/Core/Projectile/BP_Arrow.Is Enemy` (`self.isEnemy`) _current_arrow)
      (set `self.Current Arrow` null))))

(fn `UserConstructionScript`
  (`parent.UserConstructionScript`))