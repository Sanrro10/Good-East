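; BP_EnemyBruteArcher is a brute archer enemy that overrides how its parent unit responds to damage.
; Each hit plays AttackHit, reduces health and triggers death at zero.
; Surviving hits clear its ignored-enemy list, stop movement and apply knockback at a third of the incoming strength.
; Unless it is attacking, it switches state for one tick, then sets another.
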(event `self.Event Receive Damage`
  (params (Damage :type "Float (double-precision)") (KnockBackValue :type "Vector Structure"))
  (bind _charactermovement (`self.CharacterMovement`))
  (`AudioComponent.Play` (`self.AttackHit`) 0.0)
  (if (> (`self.HealthPoints`) 0.0)
    (bind _output_get (set `self.HealthPoints` (- (`self.HealthPoints`) Damage)))
    (if (<= _output_get 0.0)
      (`self.Event Die` :!label _label)
      (else
        (`KismetArrayLibrary.Array_Clear` (`self.EnemiesToIgnore`))
        (`MovementComponent.StopMovementImmediately` _charactermovement)
        (`CharacterMovementComponent.AddImpulse` _charactermovement (/ KnockBackValue (3.0 3.0 3.0)) true)
        (if (not (`self.Attacking`))
          (`self.Set State` "NewEnumerator4")
          (`KismetSystemLibrary.DelayUntilNextTick`)
          (`self.Set State` "NewEnumerator1"))))
    (else
      (goto _label))))

(fn `UserConstructionScript`
  (`parent.UserConstructionScript`))