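; Enemy archer unit that spawns a bow in its hand and gains attack range from the height of its current tile.
; DrawArrow attaches a new arrow to the hand; ShootArrow detaches it, rolls accuracy against SpecialStat, then checks the target's dodge interface.
; Hits become homing projectiles aimed at a crit-dependent target, with crits doubling damage.
; Failed shots use a suggested arc velocity toward a random point around the target.
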(event `self.ReceiveBeginPlay`
  (`parent.ReceiveBeginPlay`)
  (bind _returnvalue (`|SpawnActorFromClass` "/Game/Blueprints/Core/Weapons/BP_Bow.BP_Bow_C" (`SceneComponent.GetSocketTransform` (`self.Mesh`) "HandWeaponSocket" "RTS_World") "Undefined" "MultiplyWithRoot" null null))
  (bind _output_get (set `self.Weapon` _returnvalue))
  (`self.K2_AttachToComponent` _output_get (`self.Mesh`) "HandWeaponSocket" "SnapToTarget" "SnapToTarget" "SnapToTarget" false))

(fn `Draw Arrow`
  (bind _returnvalue (`|SpawnActorFromClass` "/Game/Blueprints/Core/Projectile/BP_Arrow.BP_Arrow_C" (`SceneComponent.GetSocketTransform` (`self.Mesh`) "HandTorchSocket" "RTS_World") "AdjustIfPossibleButAlwaysSpawn" "MultiplyWithRoot" self self))
  (bind _output_get (set `self.Current Arrow` _returnvalue))
  (`/Engine/EditorBlueprintResources/StandardMacros.IsValid` _output_get
    (:`Is Valid`
      (`self.K2_AttachToComponent` _output_get (`self.Mesh`) "HandTorchSocket" "SnapToTarget" "SnapToTarget" "SnapToTarget" false))))

(fn `Get Current Range`
  (returns (Range :type Integer))
  (return (+ (`self.Range`) (`/Game/Blueprints/Core/BP_Tile.Height` (`self.Current Tile`)))))

(fn `GetCurrentRangeInDistance`
  (returns (AttackRangeInDistance :type "Float (double-precision)"))
  (return (* (`self.Get Current Range`) 400)))

(fn `Shoot Arrow`
  (locals (`Is Crit` :type Boolean))
  (bind _current_arrow (`self.Current Arrow`))
  (bind _projectilemovement (`/Game/Blueprints/Core/Projectile/BP_Arrow.ProjectileMovement` (`self.Current Arrow`)))
  (bind _current_arrow_2 (`self.Current Arrow`)
    (:`then`
      (`self.K2_DetachFromActor` _current_arrow_2 "KeepWorld" "KeepRelative" "KeepRelative")
      (`|ExecutionSequence`
        (:`then_0`
          (if (< (`KismetMathLibrary.RandomFloatInRange` 0.0 1.0) (`self.SpecialStat`))
            (bind _attack_target_unit (`self.Attack Target Unit`)
              (:`then`
                (if (`KismetSystemLibrary.DoesImplementInterface` _attack_target_unit "/Game/Blueprints/Core/Units/Monk/BPI_Dodge.BPI_Dodge_C")
                  (bind _dodged (message `/Game/Blueprints/Core/Units/Monk/BPI_Dodge.Dodge` _attack_target_unit))
                  (if _dodged
                    (`self.Failed Shot`)
                    (else
                      (bind _output_get (set `local.Is Crit` (< (`KismetMathLibrary.RandomFloatInRange` 0.0 1.0) (`self.CritChance`))))
                      (set `ProjectileMovementComponent.HomingTargetComponent` (`self.GetArrowTarget` (`self.Attack Target Unit`) _output_get) _projectilemovement)
                      (set `ProjectileMovementComponent.bIsHomingProjectile` true _projectilemovement)))))
              (:`else`
                (`self.Failed Shot` :!label _label)))
            (else
              (goto _label))))
        (:`then_1`
          (`self.Set Arrow Damage Considering Crit` (`local.Is Crit`))
          (set `/Game/Blueprints/Core/Projectile/BP_Arrow.Is Enemy` (`self.isEnemy`) _current_arrow)
          (`ActorComponent.Activate` (`/Game/Blueprints/Core/Projectile/BP_Arrow.ProjectileMovement` _current_arrow) false)
          (set `self.Current Arrow` null))))
    (:`else`)))

(fn `UserConstructionScript`
  (`parent.UserConstructionScript`))