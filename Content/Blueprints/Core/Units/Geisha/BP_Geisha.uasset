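; Geisha unit Blueprint that fights with a BP_Fan in each hand, spawned and attached to the weapon and shield sockets on BeginPlay.
; AttackUnit stores the target and plays the attack montage unless already attacking; TargetCursed is an empty stub.
; Attack range grows with the current tile's height.
; Arrow-style projectile graphs handle homing, crit damage, and failed shots that arc randomly near the target without damage.
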(event `self.ReceiveBeginPlay`
  (`parent.ReceiveBeginPlay`)
  (bind _returnvalue (`|SpawnActorFromClass` "/Game/Blueprints/Core/Weapons/BP_Fan.BP_Fan_C" (`SceneComponent.GetSocketTransform` (`self.Mesh`) "HandWeaponSocket" "RTS_World") "Undefined" "MultiplyWithRoot" null null))
  (bind _output_get (set `self.Weapon` _returnvalue))
  (`self.K2_AttachToComponent` _output_get (`self.Mesh`) "HandWeaponSocket" "SnapToTarget" "SnapToTarget" "SnapToTarget" false)
  (bind _returnvalue_2 (`|SpawnActorFromClass` "/Game/Blueprints/Core/Weapons/BP_Fan.BP_Fan_C" (`SceneComponent.GetSocketTransform` (`self.Mesh`) "HandShieldSocket" "RTS_World") "Undefined" "MultiplyWithRoot" null null))
  (bind _output_get_2 (set `self.Seccondary Weapon` _returnvalue_2))
  (`self.K2_AttachToComponent` _output_get_2 (`self.Mesh`) "HandShieldSocket" "SnapToTarget" "SnapToTarget" "SnapToTarget" false))

(event `self.Attack Unit`
  (params (`Target Unit` :type "/Game/Blueprints/Core/Units/BP_Unit Object Reference"))
  (if (not (`self.Attacking`))
    (set `self.Attack Target Unit` `Target Unit`)
    (set `self.Attacking` true)
    (`|PlayMontage` (`self.Mesh`) (`self.Attack Montage`) (`self.Attack Play Rate`))))

(event `Event Target Cursed`)

(fn `Get Current Range`
  (returns (Range :type Integer))
  (return (+ (`self.Range`) (`/Game/Blueprints/Core/BP_Tile.Height` (`self.Current Tile`)))))

(fn `GetCurrentRangeInDistance`
  (returns (AttackRangeInDistance :type "Float (double-precision)"))
  (return (* (`self.Get Current Range`) 400)))

(fn `UserConstructionScript`
  (`parent.UserConstructionScript`))