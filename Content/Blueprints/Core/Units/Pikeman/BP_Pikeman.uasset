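; Pikeman unit Blueprint that fights with a Jumonji spear, building on a parent unit class.
; On BeginPlay it spawns BP_Jumonji at the back socket, stores it as the weapon and sets it unequipped through the parent's attachment logic.
; AttackUnit records the target and, if the weapon is equipped, plays the attack montage.
; Montage notifies toggle the spear's trail and tip Niagara effects, and blend-out clears the attacking state and signals completion.
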(event `self.ReceiveBeginPlay`
  (`parent.ReceiveBeginPlay`)
  (bind _returnvalue (`|SpawnActorFromClass` "/Game/Blueprints/Core/Weapons/BP_Jumonji.BP_Jumonji_C" (`SceneComponent.GetSocketTransform` (`self.Mesh`) "BackSocket" "RTS_World") "Undefined" "MultiplyWithRoot" null null))
  (set `self.Weapon` _returnvalue)
  (`self.SetWeaponAttachment` false))

(event `self.Attack Unit`
  (params (`Target Unit` :type "/Game/Blueprints/Core/Units/BP_Unit Object Reference"))
  (set `self.Attack Target Unit` `Target Unit`)
  (set `self.Attacking` true)
  (if (`self.Weapon Equipped`)
    (bind _notifyname (`|PlayMontage` (`self.Mesh`) (`self.Attack Montage`) (`self.Attack Play Rate`))
      (:`OnBlendOut`
        (set `self.Attacking` false)
        (`self.OnFinishAttack`))
      (:`OnNotifyBegin`
        (if (== _notifyname "Start_NSSpearTrail")
          (bind _asbp_jumonji (cast `/Game/Blueprints/Core/Weapons/BP_Jumonji` (`self.Weapon`)))
          (`/Game/Blueprints/Core/Weapons/BP_Jumonji.ToggleNSSpearTrail` _asbp_jumonji true)
          (elif (== _notifyname "Start_NSSpearTip")
            (bind _asbp_jumonji_2 (cast `/Game/Blueprints/Core/Weapons/BP_Jumonji` (`self.Weapon`)))
            (`/Game/Blueprints/Core/Weapons/BP_Jumonji.ToggleNSSpearTip` _asbp_jumonji_2 true)
            (elif (== _notifyname "Finish_NSSpearTrail")
              (bind _asbp_jumonji_3 (cast `/Game/Blueprints/Core/Weapons/BP_Jumonji` (`self.Weapon`)))
              (`/Game/Blueprints/Core/Weapons/BP_Jumonji.ToggleNSSpearTrail` _asbp_jumonji_3 false)
              (else
                (bind _asbp_jumonji_4 (cast `/Game/Blueprints/Core/Weapons/BP_Jumonji` (`self.Weapon`)))
                (`/Game/Blueprints/Core/Weapons/BP_Jumonji.ToggleNSSpearTip` _asbp_jumonji_4 false)))))))))

(fn `SetWeaponAttachment`
  (params (Equipped :type Boolean))
  (`parent.SetWeaponAttachment` Equipped))

(fn `UserConstructionScript`
  (`parent.UserConstructionScript`))