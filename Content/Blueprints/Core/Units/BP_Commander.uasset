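; BP_Commander is a squad leader unit in the defense game that spawns and leads a formation of militia, infantry, pikemen or archers.
; The construction script picks the unit class from UnitType and gathers eight formation points, where BeginPlay spawns units sharing an avoidance group from the game mode.
; MoveToTile claims the tile and sends each unit to its formation offset.
; After movement, looping timers smoothly rotate the commander and stationary units.
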(event `self.ReceiveBeginPlay`
  (bind (_avoidancegroup _groupstoavoid) (`self.Request Avoidance Groups ID`))
  (bind _output_get (set `self.Groups to Avoid` _groupstoavoid))
  (bind _output_get_2 (set `self.Avoidance Group` _avoidancegroup))
  (`CharacterMovementComponent.SetAvoidanceGroupMask` (`self.CharacterMovement`) _output_get_2)
  (`CharacterMovementComponent.SetGroupsToAvoidMask` (`self.CharacterMovement`) _output_get)
  (`CharacterMovementComponent.SetGroupsToIgnoreMask` (`self.CharacterMovement`) (`self.Avoidance Group`))
  (for _array_element (`self.SpawnPositions`)
    (bind _returnvalue (`|SpawnActorFromClass` (`self.UnitClass`) (`KismetMathLibrary.MakeTransform` (`SceneComponent.K2_GetComponentLocation` _array_element) (`self.K2_GetActorRotation`)) "AdjustIfPossibleButAlwaysSpawn" "MultiplyWithRoot" self self))
    (`KismetArrayLibrary.Array_Add` (`self.UnitsArray`) _returnvalue)
    (set `/Game/Blueprints/Core/Units/BP_Militia.FormationPosition` _array_element _returnvalue)
    (set `/Game/Blueprints/Core/Units/BP_Militia.Commander` self _returnvalue)
    (`self.Update Avoidance` _returnvalue (`self.Avoidance Group`) (`self.Groups to Avoid`))))

(fn `Move to Tile`
  (params (Tile :type "/Game/Blueprints/Core/BP_Tile Object Reference"))
  (locals (TileCenterLocation :type "Vector Structure" :default (0.0 0.0 0.0)))
  (`self.UpdateTile` Tile)
  (bind _location (`/Game/Blueprints/Core/BP_Tile.GetCenterLocation` Tile))
  (bind _output_get (set `local.TileCenterLocation` _location))
  (`self.Call Controller Move to Position` _output_get)
  (for _array_element (`self.UnitsArray`)
    (`self.Call Controller Move to Position` _array_element (+ (`SceneComponent.RelativeLocation` (`/Game/Blueprints/Core/Units/BP_Militia.FormationPosition` _array_element)) (`local.TileCenterLocation`)))))

(fn `Request Avoidance Groups ID`
  (returns (AvoidanceGroup :type "NavAvoidanceMask Structure") (GroupsToAvoid :type "NavAvoidanceMask Structure"))
  (bind _asgm_defense_game (cast `/Game/Blueprints/Core/GM_DefenseGame` (`GameplayStatics.GetGameMode`)))
  (bind (_avoidancegroup _groupstoavoid) (`/Game/Blueprints/Core/GM_DefenseGame.Get Avoidance Group ID` _asgm_defense_game))
  (return _avoidancegroup _groupstoavoid))

(fn `UpdateRotationAfterMovement`
  (set `self.DesiredRotation` (`self.GetDesiredRotation`))
  (set `self.LerpAlpha` 0.0)
  (`KismetSystemLibrary.K2_ClearTimer` null "SmoothRotation")
  (`KismetSystemLibrary.K2_SetTimer` null "SmoothRotation" 0.01 true)
  (for _array_element (`self.UnitsArray`)
    (`/Engine/EditorBlueprintResources/StandardMacros.IsValid` _array_element
      (:`Is Valid`
        (if (not (`/Game/Blueprints/Core/Units/BP_Unit.Moving` _array_element))
          (set `/Game/Blueprints/Core/Units/BP_Unit.DesiredRotation` (`self.DesiredRotation`) _array_element)
          (set `/Game/Blueprints/Core/Units/BP_Unit.LerpAlpha` 0.0 _array_element)
          (`KismetSystemLibrary.K2_ClearTimer` _array_element "SmoothRotation")
          (`KismetSystemLibrary.K2_SetTimer` _array_element "SmoothRotation" 0.01 true))))))

(fn `UpdateTile`
  (params (NewTile :type "/Game/Blueprints/Core/BP_Tile Object Reference"))
  (`/Game/Blueprints/Core/BP_Tile.SetCommander` (`self.Tile`) null)
  (bind _output_get (set `self.Tile` NewTile))
  (`/Game/Blueprints/Core/BP_Tile.SetCommander` _output_get self))

(fn `UserConstructionScript`
  (`parent.UserConstructionScript`)
  (`|ExecutionSequence`
    (:`then_0`
      (`KismetArrayLibrary.Array_Add` (`self.SpawnPositions`) (`self.FormationPosition 1`))
      (`KismetArrayLibrary.Array_Add` (`self.SpawnPositions`) (`self.FormationPosition 2`))
      (`KismetArrayLibrary.Array_Add` (`self.SpawnPositions`) (`self.FormationPosition 3`))
      (`KismetArrayLibrary.Array_Add` (`self.SpawnPositions`) (`self.FormationPosition 4`))
      (`KismetArrayLibrary.Array_Add` (`self.SpawnPositions`) (`self.FormationPosition 6`))
      (`KismetArrayLibrary.Array_Add` (`self.SpawnPositions`) (`self.FormationPosition 7`))
      (`KismetArrayLibrary.Array_Add` (`self.SpawnPositions`) (`self.FormationPosition 8`))
      (`KismetArrayLibrary.Array_Add` (`self.SpawnPositions`) (`self.FormationPosition 9`)))
    (:`then_1`
      (if (`|EnumEquality` (`self.UnitType`) "NewEnumerator0")
        (set `self.UnitClass` "/Game/Blueprints/Core/Units/BP_Militia.BP_Militia_C")
        (elif (or (`|EnumEquality` (`self.UnitType`) "NewEnumerator1") (`|EnumEquality` (`self.UnitType`) "NewEnumerator2") (`|EnumEquality` (`self.UnitType`) "NewEnumerator3"))
          (set `self.UnitClass` "/Game/Blueprints/Core/Units/BP_Infantry.BP_Infantry_C")
          (elif (or (`|EnumEquality` (`self.UnitType`) "NewEnumerator4") (`|EnumEquality` (`self.UnitType`) "NewEnumerator5") (`|EnumEquality` (`self.UnitType`) "NewEnumerator6"))
            (set `self.UnitClass` "/Game/Blueprints/Core/Units/BP_Pikeman.BP_Pikeman_C")
            (else
              (set `self.UnitClass` "/Game/Blueprints/Core/Units/BP_Archer.BP_Archer_C"))))))))