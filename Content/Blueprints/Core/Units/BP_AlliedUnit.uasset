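; Allied unit in a defense game that belongs to a Commander, extending parent unit logic for death, healing and repositioning.
; After repositioning, a looping timer lerps it toward either its yaw snapped to 90-degree steps or the Commander's facing.
; Death removes it from the Commander, then triggers repositioning of units when dying finishes.
; Entering a house teleports it to a hidden platform; reactivation after healing restarts its behavior tree with a reposition order.
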(event `SmoothRotation`
  (if (< (`self.LerpAlpha`) 1.0)
    (`self.K2_SetActorRotation` (`KismetMathLibrary.RLerp` (`self.K2_GetActorRotation`) (`self.DesiredRotation`) (`self.LerpAlpha`) true))
    (set `self.LerpAlpha` (+ (`self.LerpAlpha`) 0.01))
    (else
      (`KismetSystemLibrary.K2_ClearTimer` null "SmoothRotation")
      (`self.FinishRotating`))))

(event `self.ReceiveBeginPlay`
  (`parent.ReceiveBeginPlay`))

(event `self.Die Event`
  (`parent.Die Event`)
  (bind _commander (`self.Commander`)
    (:`then`
      (`/Game/Blueprints/Core/Units/Commander/BP_Commander.RemoveUnitFromCommander` _commander self))
    (:`else`)))

(fn `Enter House`
  (`/Game/Blueprints/Core/BP_HiddenPlatform.Teleport Onto Platform` (`/Game/Blueprints/Core/GM_DefenseGame.HiddenPlatform` (`self.GM_DefenseGame`)) self))

(fn `FinishDying`
  (`parent.FinishDying`)
  (bind _commander (`self.Commander`)
    (:`then`
      (`/Game/Blueprints/Core/Units/Commander/BP_Commander.RepositionUnits` _commander))
    (:`else`)))

(fn `GetDesiredRotation`
  (returns (DesiredRotation :type "Rotator Structure"))
  (bind (_returnvalue_roll _returnvalue_pitch _returnvalue_yaw) (`KismetMathLibrary.BreakRotator` (`self.K2_GetActorRotation`)))
  (return (`KismetMathLibrary.MakeRotator` _returnvalue_roll _returnvalue_pitch (* (`KismetMathLibrary.Round` (/ _returnvalue_yaw 90)) 90))))

(fn `Reactivate Unit After Healing`
  (params (`Desired Tile` :type "/Game/Blueprints/Core/BP_Tile Object Reference"))
  (set `self.Desired Tile` `Desired Tile`)
  (if (`/Game/Blueprints/Core/Units/AIC_Unit.Initialized BT` (`self.AIC Unit`))
    (`self.Enable Disable Behaviour Tree` true)
    (else
      (`self.Initialize Behaviour Tree`)))
  (set `self.HasRepositionOrder` true))

(fn `Update Rotation After Repositioning`
  (bind _commander (`self.Commander`))
  (if (== (`self.GetDesiredRotation`) (`self.K2_GetActorRotation`) :`ErrorTolerance` 5.0)
    (`self.K2_SetActorRotation` (`self.GetDesiredRotation`))
    (set `self.LerpAlpha` 1.0)
    (`KismetSystemLibrary.K2_SetTimer` null "SmoothRotation" 0.01)
    (else
      (`KismetSystemLibrary.K2_ClearTimer` null "SmoothRotation")
      (set `self.LerpAlpha` 0.0)
      (if (`/Game/Blueprints/Core/Units/BP_Unit.Repositioning` _commander)
        (set `self.DesiredRotation` (`self.GetDesiredRotation`))
        (else
          (set `self.DesiredRotation` (`self.GetDesiredRotation` _commander))))
      (`KismetSystemLibrary.K2_SetTimer` null "SmoothRotation" 0.01 true))))

(fn `UserConstructionScript`)