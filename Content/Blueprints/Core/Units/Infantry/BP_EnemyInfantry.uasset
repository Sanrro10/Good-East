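; BP_EnemyInfantry is an enemy infantry unit armed with a sword and shield that can block incoming arrows.
; On BeginPlay it spawns BP_Sword and BP_Shield and attaches them to the mesh's hand sockets.
; Dodge succeeds when the attacker lies within 90 degrees of facing, triggering a short timed Blocking state.
; It returns that result along with the shield's arrow target as the new target.
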(event `self.ReceiveBeginPlay`
  (`parent.ReceiveBeginPlay`)
  (bind _returnvalue (`|SpawnActorFromClass` "/Game/Blueprints/Core/Weapons/BP_Sword.BP_Sword_C" (`SceneComponent.GetSocketTransform` (`self.Mesh`) "HandWeaponSocket" "RTS_World") "Undefined" "MultiplyWithRoot" null null))
  (bind _output_get (set `self.Weapon` _returnvalue))
  (`self.K2_AttachToComponent` _output_get (`self.Mesh`) "HandWeaponSocket" "SnapToTarget" "SnapToTarget" "SnapToTarget" false)
  (bind _returnvalue_2 (`|SpawnActorFromClass` "/Game/Blueprints/Core/Weapons/BP_Shield.BP_Shield_C" (`SceneComponent.GetSocketTransform` (`self.Mesh`) "HandShieldSocket" "RTS_World") "Undefined" "MultiplyWithRoot" null null))
  (bind _output_get_2 (set `self.Shield` _returnvalue_2))
  (`self.K2_AttachToComponent` _output_get_2 (`self.Mesh`) "HandShieldSocket" "SnapToTarget" "SnapToTarget" "SnapToTarget" false))

(event `Block Arrow`
  (set `self.Blocking` true)
  (`KismetSystemLibrary.K2_SetTimerDelegate` (delegate `Stop Blocking`) 1.5))

(event `Stop Blocking`
  (set `self.Blocking` false))

(fn `Dodge`
  (params (`Attacker Position` :type "Vector Structure"))
  (returns (Dodged :type Boolean) (`New Target` :type "SceneComponent Object Reference"))
  (locals (HasDodged :type Boolean))
  (bind (_returnvalue_roll _returnvalue_pitch _returnvalue_yaw) (`KismetMathLibrary.BreakRotator` (`KismetMathLibrary.FindRelativeLookAtRotation` (`self.GetTransform`) `Attacker Position`)))
  (bind _output_get (set `local.HasDodged` (< (`KismetMathLibrary.Abs` _returnvalue_yaw) 90.0)))
  (if _output_get
    (`self.Block Arrow`))
  (return (`local.HasDodged`) (`/Game/Blueprints/Core/Weapons/BP_Shield.Get Arrow Target` (`self.Shield`))))

(fn `UserConstructionScript`
  (`parent.UserConstructionScript`))