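; Monk infantry unit that adds a chance-based dodge to its parent unit's behavior.
; The Dodge function rolls against SpecialStat, fires the dodge event on success and returns whether it dodged, ignoring the attacker's position.
; The event plays the dodge montage under a Dodging flag that blocks replays until blend-out or the first notify.
; Disconnected nodes for halting actions and movement during a dodge never run.
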(event `self.ReceiveBeginPlay`
  (`parent.ReceiveBeginPlay`))

(event `Event Dodge`
  (if (not (`self.Dodging`))
    (set `self.Dodging` true)
    (`|PlayMontage` (`self.Mesh`) "/Game/Art/Animations/Monk/Monk_Dodge_Montage.Monk_Dodge_Montage"
      (:`OnBlendOut`
        _)
      (:`OnNotifyBegin`
        _))
    (set `self.Dodging` false)))

(fn `Dodge`
  (params (`Attacker Position` :type "Vector Structure"))
  (returns (Dodged :type Boolean) (`New Target` :type "SceneComponent Object Reference"))
  (if (< (`KismetMathLibrary.RandomFloatInRange` 0.0 1.0) (`self.SpecialStat`))
    (`self.Event Dodge`)
    (return true null)
    (else
      (return false null))))

(fn `UserConstructionScript`
  (`parent.UserConstructionScript`))