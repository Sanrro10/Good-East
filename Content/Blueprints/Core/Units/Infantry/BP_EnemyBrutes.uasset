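; BP_EnemyBrutes is a brute infantry enemy, a child unit Blueprint that overrides the parent's attack, house-burning and damage handling.
; Dealing attack damage or burning a house clears CanBeInterrupted, and nothing in this file sets it back.
; Incoming hits play AttackHit, reduce health and call EventDie at zero; surviving hits clear EnemiesToIgnore.
; While interruptible, a hit also switches state, applies halved knockback and plays InterruptionMontage, restoring the previous state on blend out.
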(event `/Game/Blueprints/Core/Units/BP_EnemyUnit.Burn House`
  (params (House :type "/Game/Blueprints/Core/Houses/BP_House Object Reference"))
  (`parent.Burn House` House)
  (set `self.CanBeInterrupted` false))

(event `self.EventAttackDealDamage`
  (`parent.EventAttackDealDamage`)
  (set `self.CanBeInterrupted` false))

(event `self.Event Receive Damage`
  (params (Damage :type "Float (double-precision)") (KnockBackValue :type "Vector Structure"))
  (bind _charactermovement (`self.CharacterMovement`))
  (`AudioComponent.Play` (`self.AttackHit`) 0.0)
  (if (> (`self.HealthPoints`) 0.0)
    (bind _output_get (set `self.HealthPoints` (- (`self.HealthPoints`) Damage)))
    (if (<= _output_get 0.0)
      (`self.Event Die` :!label _label)
      (else
        (`KismetArrayLibrary.Array_Clear` (`self.EnemiesToIgnore`))
        (if (`self.CanBeInterrupted`)
          (`self.Set State` "NewEnumerator4")
          (`MovementComponent.StopMovementImmediately` _charactermovement)
          (`CharacterMovementComponent.AddImpulse` _charactermovement (/ KnockBackValue (2.0 2.0 2.0)) true)
          (`|PlayMontage` (`self.Mesh`) (`self.Interruption Montage`)
            (:`OnBlendOut`
              (`self.Set State` (`self.GetPreviousState`)))))))
    (else
      (goto _label))))

(fn `UserConstructionScript`
  (`parent.UserConstructionScript`))