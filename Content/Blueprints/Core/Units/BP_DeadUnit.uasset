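; BP_DeadUnit is a corpse stand-in that displays a dead unit as a skeletal mesh.
; Its Initialize function takes a mesh, material and animation, applies them, then makes the mesh visible.
; It sets the animation position to the clip's full length with notifies enabled, so the body shows the final pose rather than playing through.
; The event graph holds no active logic.
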(fn `Initialize`
  (params (Mesh :type "SkeletalMesh Object Reference") (Material :type "MaterialInterface Object Reference") (AnimToPlay :type "AnimationAsset Object Reference"))
  (`SkeletalMeshComponent.SetSkeletalMeshAsset` (`self.SkeletalMesh`) Mesh)
  (`PrimitiveComponent.SetMaterial` (`self.SkeletalMesh`) 0 Material)
  (`SkeletalMeshComponent.SetAnimation` (`self.SkeletalMesh`) AnimToPlay)
  (`SkeletalMeshComponent.SetPosition` (`self.SkeletalMesh`) (`AnimationAsset.GetPlayLength` AnimToPlay) true)
  (`SceneComponent.SetVisibility` (`self.SkeletalMesh`) true false))

(fn `UserConstructionScript`
  (`parent.UserConstructionScript`))