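; Base Character for allied and enemy units in a tile-based defense game, handling combat, weapon equipping, launched jumps and death.
; AIC_Unit holds state and runs the behaviour tree, while enemy searches read adjacent tiles within range.
; Montages drive attacks, hit interruptions and weapon socket swaps, with damage dealt through a bound event.
; On death it spawns a BP_DeadUnit copy, moves attached arrows onto it and destroys itself.
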(event `Event Die`
  (if (not (`self.Dying`))
    (set `self.Dying` true)
    (`|PlayMontage` (`self.Mesh`) (`self.Death Montage`)
      (:`then`
        (bind _mesh (`self.Mesh`)
          (:`then`
            (`PrimitiveComponent.SetSimulatePhysics` _mesh false)
            (`PrimitiveComponent.SetCollisionEnabled` _mesh "NoCollision")
            (`PrimitiveComponent.SetCollisionResponseToAllChannels` _mesh "ECR_Ignore")
            (set `PrimitiveComponent.CanCharacterStepUpOn` "ECB_Yes" _mesh)
            (`self.Enable Disable Behaviour Tree` false)
            (bind _aic_unit (`self.AIC Unit`)
              (:`then`
                (`/Game/Blueprints/Core/Units/AIC_Unit.Set State` _aic_unit "NewEnumerator5")
                (bind _capsulecomponent (`self.CapsuleComponent`)
                  (:`then`
                    (`PrimitiveComponent.SetSimulatePhysics` _capsulecomponent false)
                    (`PrimitiveComponent.SetCollisionEnabled` _capsulecomponent "NoCollision")
                    (`PrimitiveComponent.SetCollisionResponseToAllChannels` _capsulecomponent "ECR_Ignore")
                    (`PrimitiveComponent.SetSimulatePhysics` _capsulecomponent false)
                    (set `PrimitiveComponent.CanCharacterStepUpOn` "ECB_Yes" _capsulecomponent)
                    (bind _current_tile (`self.Current Tile`)
                      (:`then`
                        (`/Game/Blueprints/Core/BP_Tile.Remove Current Unit` _current_tile self))
                      (:`else`)))
                  (:`else`)))
              (:`else`)))
          (:`else`)))
      (:`OnBlendOut`
        (`self.FinishDying` :!label _label))
      (:`OnInterrupted`
        (goto _label)))))

(event `Event Receive Damage`
  (params (Damage :type "Float (double-precision)") (KnockBackValue :type "Vector Structure"))
  (bind _charactermovement (`self.CharacterMovement`))
  (`AudioComponent.Play` (`self.AttackHit`) 0.0)
  (if (> (`self.HealthPoints`) 0.0)
    (bind _output_get (set `self.HealthPoints` (- (`self.HealthPoints`) Damage)))
    (if (<= _output_get 0.0)
      (`self.Event Die` :!label _label_2)
      (else
        (`KismetArrayLibrary.Array_Clear` (`self.EnemiesToIgnore`))
        (if (`self.CanBeInterrupted`)
          (`self.Set State` "NewEnumerator4")
          (`MovementComponent.StopMovementImmediately` _charactermovement)
          (`CharacterMovementComponent.AddImpulse` _charactermovement KnockBackValue true)
          (`|PlayMontage` (`self.Mesh`) (`self.Interruption Montage`)
            (:`OnBlendOut`
              (`self.Set State` (`self.GetPreviousState`)))))))
    (else
      (goto _label_2))))

(event `self.ReceivePossessed`
  (params (NewController :type "Controller Object Reference"))
  (bind _asaic_unit (cast `/Game/Blueprints/Core/Units/AIC_Unit` NewController))
  (bind _output_get (set `self.AIC Unit` _asaic_unit))
  ;[1 0.4673 0] Debug
  (`self.K2_AttachToComponent` _output_get (`self.CapsuleComponent`) "HandWeaponSocket" "SnapToTarget" "SnapToTarget" "SnapToTarget" false)
  (if (`self.StartWithBehaviourTreeEnabled`)
    (`self.Initialize Behaviour Tree`)))

(event `Event Equip Weapon`
  (`|PlayMontage` (`self.Mesh`) (`self.Weapon Equip Montage`)
    (:`OnInterrupted`
      _)
    (:`OnNotifyBegin`
      _))
  (`self.SetWeaponAttachment` true)
  (`self.OnWeaponEquipped`))

(event `Event Unequip Weapon`
  (`|PlayMontage` (`self.Mesh`) (`self.Weapon Unequip Montage`)
    (:`OnBlendOut`
      (`self.OnWeaponUnequipped`))
    (:`OnInterrupted`
      (`self.SetWeaponAttachment` false)
      (`self.OnWeaponUnequipped`))
    (:`OnNotifyBegin`
      (`self.SetWeaponAttachment` false))))

(event `Attack Unit`
  (params (`Target Unit` :type "/Game/Blueprints/Core/Units/BP_Unit Object Reference"))
  (if (not (`self.Attacking`))
    (set `self.Attack Target Unit` `Target Unit`)
    (set `self.Attacking` true)
    (if (`self.Weapon Equipped`)
      (`|PlayMontage` (`self.Mesh`) (`self.Attack Montage`) (`self.Attack Play Rate`)
        (:`OnBlendOut`
          (set `self.Attacking` false)
          (`self.OnFinishAttack`))))))

(event `self.ReceiveBeginPlay`
  (`parent.ReceiveBeginPlay`)
  (add `self.OnAttackDealDamage` (delegate `EventAttackDealDamage`))
  (add `self.OnSetIninterrumpible` (delegate `SetininterrumpibleEvent`))
  (bind _asgm_defense_game (cast `/Game/Blueprints/Core/GM_DefenseGame` (`GameplayStatics.GetGameMode`)))
  (set `self.GM_DefenseGame` _asgm_defense_game))

(event `EventAttackDealDamage`
  (bind _attack_target_unit (`self.Attack Target Unit`))
  (`/Engine/EditorBlueprintResources/StandardMacros.IsValid` _attack_target_unit
    (:`Is Valid`
      (`self.Event Receive Damage` _attack_target_unit (`self.Attack Damage`) (0.0 0.0 0.0)))
    (:`Is Not Valid`
      _))
  (set `self.CanBeInterrupted` true))

(event `SetininterrumpibleEvent`
  (set `self.CanBeInterrupted` false))

(event `Event Jump To Destination`
  (params (Destination :type "Vector Structure"))
  (bind _outlaunchvelocity (`GameplayStatics.SuggestProjectileVelocity_CustomArc` (`self.K2_GetActorLocation`) (`KismetMathLibrary.MakeVector` Destination_X Destination_Y (+ Destination_Z (`CapsuleComponent.CapsuleHalfHeight` (`self.CapsuleComponent`))))))
  (`self.LaunchCharacter` _outlaunchvelocity true true)
  (set `self.Being Launched` true))

(event `self.OnLanded`
  (params (Hit :type "HitResult Structure (by ref)"))
  (if (`self.Being Launched`)
    (`self.Set State` "NewEnumerator0")
    (set `self.Being Launched` false)))

(fn `Add Attacker`
  (params (Attacker :type "/Game/Blueprints/Core/Units/BP_Unit Object Reference (by ref)"))
  (`KismetArrayLibrary.Array_AddUnique` (`self.Attackers`) Attacker))

(fn `Enable Disable Behaviour Tree`
  (params (Enable :type Boolean))
  (locals (`Brain Component` :type "BrainComponent Object Reference"))
  (bind _aic_unit (`self.AIC Unit`)
    (:`then`
      (bind _braincomponent (`AIController.BrainComponent` _aic_unit)
        (:`then`
          (set `local.Brain Component` _braincomponent)
          (if Enable
            (`BrainComponent.RestartLogic` (`local.Brain Component`))
            (else
              (`NavMovementComponent.StopActiveMovement` (`self.CharacterMovement`))
              (`BrainComponent.StopLogic` (`local.Brain Component`) ""))))
        (:`else`)))
    (:`else`)))

(fn `FinishDying`
  (bind _mesh (`self.Mesh`))
  (bind _animationdata_animtoplay (break `SingleAnimationPlayData` (`SkeletalMeshComponent.AnimationData` _mesh)))
  (`SkeletalMeshComponent.SetAnimationMode` (`self.Mesh`) "AnimationSingleNode" true)
  (bind _returnvalue (`|SpawnActorFromClass` "/Game/Blueprints/Core/Units/BP_DeadUnit.BP_DeadUnit_C" (`SceneComponent.K2_GetComponentToWorld` (`self.Mesh`)) "AlwaysSpawn" "MultiplyWithRoot" null null))
  (`/Engine/EditorBlueprintResources/StandardMacros.IsValid` _returnvalue
    (:`Is Valid`
      (`/Game/Blueprints/Core/Units/BP_DeadUnit.Initialize` _returnvalue (`SkeletalMeshComponent.SkeletalMeshAsset` _mesh) (`PrimitiveComponent.GetMaterial` _mesh 0) _animationdata_animtoplay)
      (`/Game/Blueprints/Core/Units/BP_DeadUnit.Initialize` _returnvalue (`SkeletalMeshComponent.SkeletalMeshAsset` _mesh) (`PrimitiveComponent.GetMaterial` _mesh 0) _animationdata_animtoplay)
      (for _array_element (`self.GetAttachedActors` true true)
        (bind _asbp_arrow (cast `/Game/Blueprints/Core/Projectile/BP_Arrow` _array_element))
        (`self.K2_AttachToComponent` _asbp_arrow (`/Game/Blueprints/Core/Units/BP_DeadUnit.SkeletalMesh` _returnvalue) (`self.GetAttachParentSocketName` _asbp_arrow) "SnapToTarget" "KeepWorld" "KeepWorld" true)
        (`SceneComponent.SetMobility` (`/Game/Blueprints/Core/Projectile/BP_Arrow.StaticMesh` _asbp_arrow) "Static"))
      (`self.K2_DestroyActor`))))

(fn `Get Attackers`
  (returns (Attackers :type "Array of /Game/Blueprints/Core/Units/BP_Unit Object Reference"))
  (bind _attackers (`self.Attackers`))
  (for (_array_element _array_index) _attackers
    (`/Engine/EditorBlueprintResources/StandardMacros.IsValid` _array_element
      (:`Is Not Valid`
        (`KismetArrayLibrary.Array_Remove` (`self.Attackers`) _array_index))))
  (return _attackers))

(fn `Get Current Range`
  (returns (Range :type Integer))
  (return (`self.Range`)))

(fn `GetArrowTarget`
  (params (IsHead :type Boolean))
  (returns (`Target Component` :type "SceneComponent Object Reference"))
  (if IsHead
    (return (`self.HeadPosition`))
    (else
      (switch `int` (`KismetMathLibrary.RandomIntegerInRange` 0 4)
        (:`Default`
          _)
        (:`0`
          (return (`self.BodyPosition1`)))
        (:`1`
          (return (`self.BodyPosition2`)))
        (:`2`
          (return (`self.BodyPosition3`)))
        (:`3`
          (return (`self.BodyPosition4`)))
        (:`4`
          _))
      (return (`self.BodyPosition5`)))))

(fn `GetCurrentRangeInDistance`
  (returns (AttackRangeInDistance :type "Float (double-precision)"))
  (return (`self.AttackRangeInDistance`)))

(fn `GetCurrentState`
  (returns (State :type "/Game/Structures+Enumerators/EUnitStates Enum"))
  (bind _aic_unit (`self.AIC Unit`)
    (:`then`
      (return (`/Game/Blueprints/Core/Units/AIC_Unit.Get Current State` _aic_unit)))
    (:`else`
      (return "NewEnumerator0"))))

(fn `GetIsDamaged`
  (returns (Damaged :type Boolean))
  (return (== (`self.MaxHealthPoints`) (`self.HealthPoints`))))

(fn `GetIsDead`
  (returns (IsDead :type Boolean))
  (bind _aic_unit (`self.AIC Unit`)
    (:`then`
      (return (`|EnumEquality` (`/Game/Blueprints/Core/Units/AIC_Unit.Get Current State` _aic_unit) "NewEnumerator5")))
    (:`else`
      (return true))))

(fn `GetPreviousState`
  (returns (State :type "/Game/Structures+Enumerators/EUnitStates Enum"))
  (return (`/Game/Blueprints/Core/Units/AIC_Unit.GetPreviousState` (`self.AIC Unit`))))

(fn `Initialize Behaviour Tree`
  (bind _aic_unit (`self.AIC Unit`)
    (:`then`
      (`/Game/Blueprints/Core/Units/AIC_Unit.Initialize Behaviour Tree` _aic_unit self))
    (:`else`
      (set `self.StartWithBehaviourTreeEnabled` true))))

(fn `Look for Enemies Around Current Tile`
  (returns (EnemiesAroundCurrentTile :type "Array of /Game/Blueprints/Core/Units/BP_Unit Object Reference"))
  (locals (EnemiesAroundCurrentTileArray :type "Array of /Game/Blueprints/Core/Units/BP_Unit Object Reference"))
  (bind _current_tile (`self.Current Tile`)
    (:`then`
      (bind _adjacent_tiles (`/Game/Blueprints/Core/BP_Tile.Get Adjacent Tiles` _current_tile (`self.Get Current Range`)))
      (if (`self.isEnemy`)
        (for _array_element _adjacent_tiles
          (for _array_element_2 (`/Game/Blueprints/Core/BP_Tile.AlliesCurrentlyOnTile` _array_element)
            (`KismetArrayLibrary.Array_AddUnique` (`local.EnemiesAroundCurrentTileArray`) _array_element_2)))
        (else
          (for _array_element_3 _adjacent_tiles
            (for _array_element_4 (`/Game/Blueprints/Core/BP_Tile.EnemiesCurrentlyOnTile` _array_element_3)
              (`KismetArrayLibrary.Array_AddUnique` (`local.EnemiesAroundCurrentTileArray`) _array_element_4)))))
      (return (`local.EnemiesAroundCurrentTileArray`)))
    (:`else`
      (`KismetSystemLibrary.PrintString` (`KismetStringLibrary.Concat_StrStr` "ERROR: NULL CURRENT TILE ON " (`KismetSystemLibrary.GetDisplayName` self) " WHEN TRYING TO GET ENEMIES IN RANGE") true true (struct :`R` 0.995 :`G` 0.016 :`A` 1.0) 10.0)
      (return (`local.EnemiesAroundCurrentTileArray`)))))

(fn `Look for Enemies Around Desired Tile`
  (returns (EnemiesAroundCurrentTile :type "Array of /Game/Blueprints/Core/Units/BP_Unit Object Reference"))
  (locals (EnemiesAroundCurrentTileArray :type "Array of /Game/Blueprints/Core/Units/BP_Unit Object Reference"))
  (bind _adjacent_tiles (`/Game/Blueprints/Core/BP_Tile.Get Adjacent Tiles` (`self.Desired Tile`) (`self.Get Current Range`)))
  (if (`self.isEnemy`)
    (for _array_element _adjacent_tiles
      (for _array_element_2 (`/Game/Blueprints/Core/BP_Tile.AlliesCurrentlyOnTile` _array_element)
        (`KismetArrayLibrary.Array_AddUnique` (`local.EnemiesAroundCurrentTileArray`) _array_element_2)))
    (else
      (for _array_element_3 _adjacent_tiles
        (for _array_element_4 (`/Game/Blueprints/Core/BP_Tile.EnemiesCurrentlyOnTile` _array_element_3)
          (`KismetArrayLibrary.Array_AddUnique` (`local.EnemiesAroundCurrentTileArray`) _array_element_4)))))
  (return (`local.EnemiesAroundCurrentTileArray`)))

(fn `Play Steps`
  (`AudioComponent.Play` (`self.StepsAudio`) 0.0))

(fn `Remove Attacker`
  (params (Attacker :type "/Game/Blueprints/Core/Units/BP_Unit Object Reference (by ref)"))
  (`KismetArrayLibrary.Array_RemoveItem` (`self.Attackers`) Attacker))

(fn `Set State`
  (params (NewState :type "/Game/Structures+Enumerators/EUnitStates Enum" :default "NewEnumerator0"))
  (bind _aic_unit (`self.AIC Unit`)
    (:`then`
      (`/Game/Blueprints/Core/Units/AIC_Unit.Set State` _aic_unit NewState))
    (:`else`)))

(fn `SetWeaponAttachment`
  (params (Equipped :type Boolean))
  (bind _output_get (set `self.Weapon Equipped` Equipped))
  (if _output_get
    (`self.K2_AttachToComponent` (`self.Weapon`) (`self.Mesh`) "HandWeaponSocket" "SnapToTarget" "SnapToTarget" "SnapToTarget" false)
    (`self.OnWeaponEquipped`)
    (else
      (`self.K2_AttachToComponent` (`self.Weapon`) (`self.Mesh`) "BackSocket" "SnapToTarget" "SnapToTarget" "SnapToTarget" false)
      (`self.OnWeaponUnequipped`))))

(fn `SetWeaponVisibility`
  (params (Visible :type Boolean))
  (`self.SetActorHiddenInGame` (`self.Weapon`) (not Visible)))

(fn `Update Avoidance`
  (params (AvoidanceGroup :type "NavAvoidanceMask Structure") (GroupsToAvoid :type "NavAvoidanceMask Structure") (GroupsToIgnore :type "NavAvoidanceMask Structure"))
  (`CharacterMovementComponent.SetAvoidanceGroupMask` (`self.CharacterMovement`) AvoidanceGroup)
  (`CharacterMovementComponent.SetGroupsToAvoidMask` (`self.CharacterMovement`) GroupsToAvoid)
  (`CharacterMovementComponent.SetGroupsToIgnoreMask` (`self.CharacterMovement`) GroupsToIgnore))

(fn `UserConstructionScript`
  (`parent.UserConstructionScript`)
  (set `self.HealthPoints` (`KismetMathLibrary.Conv_IntToDouble` (`self.MaxHealthPoints`)))
  (`SceneComponent.K2_AttachToComponent` (`self.HeadPosition`) (`self.Mesh`) "headSocket" "KeepRelative" "KeepRelative" "KeepRelative" true)
  (`SceneComponent.K2_AttachToComponent` (`self.BodyPosition1`) (`self.Mesh`) "UpperArm_RSocket" "KeepRelative" "KeepRelative" "KeepRelative" true)
  (`SceneComponent.K2_AttachToComponent` (`self.BodyPosition2`) (`self.Mesh`) "UpperArm_LSocket" "KeepRelative" "KeepRelative" "KeepRelative" true)
  (`SceneComponent.K2_AttachToComponent` (`self.BodyPosition3`) (`self.Mesh`) "spine_01Socket" "KeepRelative" "KeepRelative" "KeepRelative" true)
  (`SceneComponent.K2_AttachToComponent` (`self.BodyPosition4`) (`self.Mesh`) "spine_02Socket" "KeepRelative" "KeepRelative" "KeepRelative" true)
  (`SceneComponent.K2_AttachToComponent` (`self.BodyPosition5`) (`self.Mesh`) "Thigh_LSocket" "KeepRelative" "KeepRelative" "KeepRelative" true))