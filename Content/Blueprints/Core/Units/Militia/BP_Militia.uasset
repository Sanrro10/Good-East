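; BP_Militia is a militia unit Blueprint that equips itself with an odachi when play begins.
; After running the parent BeginPlay, it spawns a BP_Odachi at the mesh's right-hand socket, stores the reference and snaps the weapon to that socket.
; The construction script only calls its parent, and the Tick and overlap events are disabled placeholders.
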(event `self.ReceiveBeginPlay`
  (`parent.ReceiveBeginPlay`)
  (bind _returnvalue (`|SpawnActorFromClass` "/Game/Blueprints/Core/Weapons/BP_Odachi.BP_Odachi_C" (`SceneComponent.GetSocketTransform` (`self.Mesh`) "HandR_Odachi_Socket" "RTS_World") "Undefined" "MultiplyWithRoot" null null))
  (bind _output_get (set `self.Odachi` _returnvalue))
  (`self.K2_AttachToComponent` _output_get (`self.Mesh`) "HandR_Odachi_Socket" "SnapToTarget" "SnapToTarget" "SnapToTarget" false))

(fn `UserConstructionScript`
  (`parent.UserConstructionScript`))