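; Player camera for the defense game that rotates, zooms, pauses and handles mouse selection and movement of commanders.
; Registers with GM_DefenseGame; zoom interpolates field of view on Tick, which is enabled after level start and disables itself at the target.
; Click traces select commanders via tiles or units, then move or reposition them, toggling tile display through the game mode.
; Debug keys damage allied units and change time dilation.
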(event `Start Level`
  (set `self.LevelStarted` true))

(event `self.ReceiveBeginPlay`
  (bind _asdefense_game_player_controller (cast `DefenseGamePlayerController` (`GameplayStatics.GetPlayerController` 0))
    (:`then`
      (bind _returnvalue (pcsubsystem `EnhancedInputLocalPlayerSubsystem` _asdefense_game_player_controller))
      (`/Engine/EditorBlueprintResources/StandardMacros.IsValid` _returnvalue
        (:`Is Valid`
          (`EnhancedInputSubsystemInterface.AddMappingContext` _returnvalue "/Game/Input/IMC_Default.IMC_Default" 0 (struct)))
        (:`Is Not Valid`
          (`KismetSystemLibrary.PrintString` "ERROR: Input system not valid" true true (struct :`R` 1.0 :`G` 0.032916 :`A` 1.0)))))
    (:`CastFailed`
      (`KismetSystemLibrary.PrintString` "ERROR: PlayerController Cast Failed" true true (struct :`R` 1.0 :`G` 0.032916 :`A` 1.0))))
  (set `self.Zoom_Desired` (`CameraComponent.FieldOfView` (`self.Camera`)))
  (bind _asgm_defense_game (cast `/Game/Blueprints/Core/GM_DefenseGame` (`GameplayStatics.GetGameMode`))
    (:`then`
      (set `/Game/Blueprints/Core/GM_DefenseGame.PlayerCamera` self _asgm_defense_game)
      (bind _output_get (set `self.As GM Defense Game` _asgm_defense_game))
      (add `/Game/Blueprints/Core/GM_DefenseGame.StartLevel` _output_get (delegate `Start Level`)))
    (:`CastFailed`
      (`KismetSystemLibrary.PrintString` "ERROR: Active Game mode is not GM_DefenseGame" true true (struct :`R` 1.0 :`G` 0.032916 :`A` 1.0)))))

(event `EnhancedInput|/Game/Input/Actions/IA_ZoomCamera`
  (params (ActionValue :type "Float (double-precision)") (ElapsedSeconds :type "Float (double-precision)") (TriggeredSeconds :type "Float (double-precision)") (InputAction :type "InputAction Object Reference" :default "/Game/Input/Actions/IA_ZoomCamera.IA_ZoomCamera"))
  ;[1 0.3281 0] Camera Zoom
  (:`Triggered`
    (set `self.Zoom_Desired` (`KismetMathLibrary.FClamp` (+ (* ActionValue 20.0) (`CameraComponent.FieldOfView` (`self.Camera`))) 40.0 100.0))
    (`self.SetActorTickEnabled` (`self.LevelStarted`))))

(event `EnhancedInput|/Game/Input/Actions/IA_RotateCamera`
  (params (ActionValue :type "Float (double-precision)") (ElapsedSeconds :type "Float (double-precision)") (TriggeredSeconds :type "Float (double-precision)") (InputAction :type "InputAction Object Reference" :default "/Game/Input/Actions/IA_RotateCamera.IA_RotateCamera"))
  (bind (_returnvalue_roll _returnvalue_pitch _returnvalue_yaw) (`KismetMathLibrary.BreakRotator` (`self.K2_GetActorRotation`)))
  ;[0.05469 0 1] Camera Rotation
  (:`Triggered`
    (`self.K2_SetActorRotation` (`KismetMathLibrary.MakeRotator` _returnvalue_roll _returnvalue_pitch (+ _returnvalue_yaw (* ActionValue (`self.CameraRotationSensibility`)))))))

(event `self.ReceiveTick`
  (params (DeltaSeconds :type "Float (single-precision)"))
  (bind _fieldofview (`CameraComponent.FieldOfView` (`self.Camera`)))
  ;[1 0.3281 0] Camera Zoom
  (if (== (`self.Zoom_Desired`) _fieldofview)
    (`self.SetActorTickEnabled` false)
    (else
      (`CameraComponent.SetFieldOfView` (`self.Camera`) (`KismetMathLibrary.FInterpTo` _fieldofview (`self.Zoom_Desired`) DeltaSeconds 2.0)))))

(event `EnhancedInput|/Game/Input/Actions/IA_PauseGame`
  (params (ActionValue :type Boolean) (ElapsedSeconds :type "Float (double-precision)") (TriggeredSeconds :type "Float (double-precision)") (InputAction :type "InputAction Object Reference" :default "/Game/Input/Actions/IA_PauseGame.IA_PauseGame"))
  ;[1 0.07031 0] Pause
  (:`Triggered`
    (`self.PauseGame`)))

(event `EnhancedInput|/Game/Input/Actions/IA_DragRotateCamera`
  (params (ActionValue :type "Float (double-precision)") (ElapsedSeconds :type "Float (double-precision)") (TriggeredSeconds :type "Float (double-precision)") (InputAction :type "InputAction Object Reference" :default "/Game/Input/Actions/IA_DragRotateCamera.IA_DragRotateCamera"))
  (bind (_returnvalue_roll _returnvalue_pitch _returnvalue_yaw) (`KismetMathLibrary.BreakRotator` (`self.K2_GetActorRotation`)))
  ;[0.05469 0 1] Camera Rotation
  (:`Triggered`
    (set `self.NewLocation` (`PlayerController.GetMousePosition` (`GameplayStatics.GetPlayerController` 0)))
    (`self.K2_SetActorRotation` (`KismetMathLibrary.MakeRotator` _returnvalue_roll _returnvalue_pitch (+ _returnvalue_yaw (/ (- (`self.NewLocation`) (`self.PreviousLocation`)) 6.0))))
    (set `self.PreviousLocation` (`PlayerController.GetMousePosition` (`GameplayStatics.GetPlayerController` 0))))
  (:`Started`
    (set `self.PreviousLocation` (`PlayerController.GetMousePosition` (`GameplayStatics.GetPlayerController` 0)))))

(event `EnhancedInput|/Game/Input/Actions/IA_SetDestination_Click`
  (params (ActionValue :type Boolean) (ElapsedSeconds :type "Float (double-precision)") (TriggeredSeconds :type "Float (double-precision)") (InputAction :type "InputAction Object Reference" :default "/Game/Input/Actions/IA_SetDestination_Click.IA_SetDestination_Click"))
  (bind _selectedcommander (`self.SelectedCommander`))
  (bind (_worldlocation _worlddirection) (`PlayerController.DeprojectMousePositionToWorld` (`GameplayStatics.GetPlayerController` 0)))
  (:`Started`
    (bind (_outhit _returnvalue) (`KismetSystemLibrary.LineTraceSingle` _worldlocation (+ _worldlocation (* _worlddirection 10000)) "TraceTypeQuery1" true))
    (if _returnvalue
      (bind (_bblockinghit _binitialoverlap _time _distance _location _impactpoint _normal _impactnormal _physmat _hitactor) (`GameplayStatics.BreakHitResult` _outhit))
      (bind _asbp_tile (cast `/Game/Blueprints/Core/BP_Tile` _hitactor)
        (:`then`
          (bind _type (`/Game/Blueprints/Core/BP_Tile.Type` _asbp_tile))
          (if (and (`|EnumInequality` "NewEnumerator2" _type) (`|EnumInequality` _type "NewEnumerator1") (`|EnumInequality` _type "NewEnumerator7"))
            (`/Engine/EditorBlueprintResources/StandardMacros.IsValid` _selectedcommander
              (:`Is Valid`
                (bind _type_2 (`/Game/Blueprints/Core/BP_Tile.Type` _asbp_tile))
                (if (or (`|EnumEquality` "NewEnumerator6" _type_2) (`|EnumEquality` _type_2 "NewEnumerator5"))
                  (if (`/Game/Blueprints/Core/BP_Tile.Get Can House be Selected` _asbp_tile)
                    (`/Game/Blueprints/Core/Units/Commander/BP_Commander.Move to Tile` _selectedcommander _asbp_tile :!label _label)
                    (`/Game/Blueprints/Core/GM_DefenseGame.HideTiles` (`self.As GM Defense Game`))
                    (set `self.SelectedCommander` null)
                    (else
                      (`KismetSystemLibrary.PrintString` "HOUSE NOT EMPTY")))
                  (else
                    (goto _label))))
              (:`Is Not Valid`
                (bind _commander (`/Game/Blueprints/Core/BP_Tile.Commander` _asbp_tile))
                (`/Engine/EditorBlueprintResources/StandardMacros.IsValid` _commander
                  (:`Is Valid`
                    (if (`/Game/Blueprints/Core/Units/Commander/BP_Commander.Can Be Selected` _commander)
                      (bind _output_get (set `self.SelectedCommander` _commander))
                      (`/Game/Blueprints/Core/GM_DefenseGame.ShowTiles` (`self.As GM Defense Game`) _output_get))))))))
        (:`CastFailed`
          (`self.Handle Commander Selection` _hitactor
            (:`To Show Tiles`
              (`/Game/Blueprints/Core/GM_DefenseGame.HideTiles` (`self.As GM Defense Game`))
              (set `self.SelectedCommander` null))
            (:`To Hide Tiles`
              (`/Game/Blueprints/Core/GM_DefenseGame.ShowTiles` (`self.As GM Defense Game`) (`self.SelectedCommander`)))
            (:`CastFailed`
              (bind _asbp_unit (cast `/Game/Blueprints/Core/Units/BP_Unit` _hitactor))
              (`self.Handle Commander Selection` (`self.GetInstigator` _asbp_unit)
                (:`To Show Tiles`
                  (`/Game/Blueprints/Core/GM_DefenseGame.HideTiles` (`self.As GM Defense Game`))
                  (set `self.SelectedCommander` null))
                (:`To Hide Tiles`
                  (`/Game/Blueprints/Core/GM_DefenseGame.ShowTiles` (`self.As GM Defense Game`) (`self.SelectedCommander`)))))))))))

(event `Key|ñ`
  (params (Key :type "Key Structure"))
  ;[1 0.868 0] DEBUG
  (:`Pressed`
    (bind _outactors (`GameplayStatics.GetAllActorsOfClass` "/Game/Blueprints/Core/Units/BP_AlliedUnit.BP_AlliedUnit_C"))
    (for _array_element _outactors
      (if (!= (`GameplayStatics.GetObjectClass` _array_element) "/Game/Blueprints/Core/Units/Commander/BP_Commander.BP_Commander_C")
        (`/Game/Blueprints/Core/Units/BP_Unit.Event Receive Damage` _array_element 4.0 (0.0 0.0 0.0))))))

(event `Key|C_Cedille`
  (params (Key :type "Key Structure"))
  ;[1 0.868 0] DEBUG
  (:`Pressed`
    (bind _outactors (`GameplayStatics.GetAllActorsOfClass` "/Game/Blueprints/Core/Units/Commander/BP_Commander.BP_Commander_C"))
    (if (`KismetArrayLibrary.Array_IsNotEmpty` _outactors)
      (`/Game/Blueprints/Core/Units/BP_Unit.Event Receive Damage` (`KismetArrayLibrary.Array_Random` _outactors) 4.0 (0.0 0.0 0.0)))))

(event `Key|RightMouseButton`
  (params (Key :type "Key Structure"))
  ;[1 0.868 0] DEBUG
  (:`Pressed`
    (`GameplayStatics.SetGlobalTimeDilation` 3.0))
  (:`Released`
    (`GameplayStatics.SetGlobalTimeDilation` 1.0)))

(event `Key|A`
  (params (Key :type "Key Structure"))
  ;[1 0.868 0] DEBUG
  (:`Pressed`
    (`/Engine/EditorBlueprintResources/StandardMacros.FlipFlop`
      (:`A`
        (`GameplayStatics.SetGlobalTimeDilation` 0.25))
      (:`B`
        (`GameplayStatics.SetGlobalTimeDilation` 1.0)))))

(fn `PauseGame`
  (`GameplayStatics.SetGamePaused` true)
  (bind _returnvalue (`|CreateWidget` "/Game/Blueprints/Widgets/SubMenus/WBP_PauseMenu.WBP_PauseMenu_C"))
  (`UserWidget.AddToViewport` _returnvalue 0))

(fn `UnpauseGame`
  (`GameplayStatics.SetGamePaused` false))

(fn `UserConstructionScript`
  (`self.K2_SetActorLocationAndRotation` (200.0 200.0 2500.0)))