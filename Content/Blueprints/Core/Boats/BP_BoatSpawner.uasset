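; BP_BoatSpawner is an actor that spawns boats at its own transform.
; AddBoatToQueue appends a boat class to BoatQueue and immediately calls SpawnBoat, which always spawns BP_Boat and returns it with a Destination.
; The queue is never consumed: its validity check, removal and Move call are disconnected, as is a Sphere overlap check, so the queued class has no effect on spawning.
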(fn `AddBoatToQueue`
  (params (BoatClass :type "/Game/Blueprints/Core/Boats/BP_Boat Class Reference (by ref)"))
  (`KismetArrayLibrary.Array_Add` (`self.BoatQueue`) BoatClass)
  (`self.SpawnBoat`))

(fn `SpawnBoat`
  (returns (Success :type Boolean) (Boat :type "Pawn Object Reference") (Destination :type "Vector Structure"))
  (bind _returnvalue (`|SpawnActorFromClass` "/Game/Blueprints/Core/Boats/BP_Boat.BP_Boat_C" (`self.GetTransform`) "Undefined" "MultiplyWithRoot" null null))
  (return true _returnvalue (`self.Destination`)))

(fn `UserConstructionScript`)