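; BP_BoatSmall is a small boat Blueprint that sets the order in which its carried units jump off when disembarking.
; GetNextUnitToJump maps the DisembarkedUnits count through a hard-coded switch to an index in UnitsArray and returns that unit.
; Only the second and third jumps pick a non-zero index; all others take the first element.
; The event graph is unused and the construction script just calls its parent.
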(fn `Get Next Unit To Jump`
  (returns (`Unit ` :type "/Game/Blueprints/Core/Units/BP_EnemyUnit Object Reference"))
  (`|ExecutionSequence`
    (:`then_0`
      (switch `int` (`self.Disembarked Units`)
        (:`Default`
          (set `self.Unit To Jump Index` 0))
        (:`0`
          (set `self.Unit To Jump Index` 0))
        (:`1`
          (set `self.Unit To Jump Index` 2))
        (:`2`
          (set `self.Unit To Jump Index` 1))
        (:`3`
          (set `self.Unit To Jump Index` 0))
        (:`4`
          (set `self.Unit To Jump Index` 0))
        (:`5`
          (set `self.Unit To Jump Index` 0))
        (:`6`
          (set `self.Unit To Jump Index` 0))
        (:`7`
          (set `self.Unit To Jump Index` 0))
        (:`8`
          (set `self.Unit To Jump Index` 0))))
    (:`then_1`
      (return (`|GetArrayItem` (`self.Units Array`) (`self.Unit To Jump Index`))))))

(fn `UserConstructionScript`
  (`parent.UserConstructionScript`))