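; BP_Shield is a shield actor that varies its appearance and supplies target points for arrows.
; The construction script gives its static mesh a random mesh from ShieldMeshes and a random material from ShieldMaterials in slot 0.
; GetArrowTarget returns one of eleven ShieldPosition references at random, presumably so arrows land at varied spots on the shield.
; The event graph holds only disabled default events.
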(fn `Get Arrow Target`
  (returns (`Target Component` :type "SceneComponent Object Reference"))
  (switch `int` (`KismetMathLibrary.RandomIntegerInRange` 1 11)
    (:`Default`
      _)
    (:`1`
      (return (`self.Shield Position 1`)))
    (:`2`
      (return (`self.Shield Position 2`)))
    (:`3`
      (return (`self.Shield Position 3`)))
    (:`4`
      (return (`self.Shield Position 4`)))
    (:`5`
      (return (`self.Shield Position 5`)))
    (:`6`
      (return (`self.Shield Position 6`)))
    (:`7`
      (return (`self.Shield Position 7`)))
    (:`8`
      (return (`self.Shield Position 8`)))
    (:`9`
      (return (`self.Shield Position 9`)))
    (:`10`
      (return (`self.Shield Position 10`)))
    (:`11`
      _))
  (return (`self.Shield Position 11`)))

(fn `UserConstructionScript`
  (bind _staticmesh (`self.StaticMesh`))
  (`parent.UserConstructionScript`)
  (`StaticMeshComponent.SetStaticMesh` _staticmesh (`KismetArrayLibrary.Array_Random` (`self.Shield Meshes`)))
  (`PrimitiveComponent.SetMaterial` _staticmesh 0 (`KismetArrayLibrary.Array_Random` (`self.Shield Materials`))))