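; BP_Jumonji is a spear weapon Blueprint that exposes switches for its tip and trail effects.
; ToggleNSSpearTip and ToggleNSSpearTrail each activate, with reset, or deactivate their effect component from a boolean.
; The event graph and construction script do nothing.
; A disconnected "OLD VFX" block remains, which sized and aligned a ribbon using the mesh's top and bottom sockets.
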(fn `ToggleNSSpearTip`
  (params (Activate :type Boolean))
  (if Activate
    (`ActorComponent.Activate` (`self.NS_SpearTip`) true)
    (else
      (`ActorComponent.Deactivate` (`self.NS_SpearTip`)))))

(fn `ToggleNSSpearTrail`
  (params (Activate :type Boolean))
  (if Activate
    (`ActorComponent.Activate` (`self.NS_SpearTrail`) true)
    (else
      (`ActorComponent.Deactivate` (`self.NS_SpearTrail`)))))

(fn `UserConstructionScript`)