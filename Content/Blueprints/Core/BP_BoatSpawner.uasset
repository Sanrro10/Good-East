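; BP_BoatSpawner is an actor that spawns boats from a class queue and sends them toward a destination.
; AddBoatToQueue appends a boat class and immediately calls SpawnBoat.
; SpawnBoat spawns the first queued class at the spawner's transform, calls Move toward Destination at the spawner's height, then dequeues it and reports success.
; A Sphere overlap check is left unconnected, so spawning never waits for clear space.
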(fn `AddBoatToQueue`
  (params (BoatClass :type "/Game/Blueprints/Core/BP_Boat Class Reference (by ref)"))
  (`KismetArrayLibrary.Array_Add` (`self.BoatQueue`) BoatClass)
  (`self.SpawnBoat`))

(fn `SpawnBoat`
  (returns (Success :type Boolean))
  (bind _returnvalue (`self.GetTransform`))
  (bind (_destination_x _destination_y) (`KismetMathLibrary.BreakVector` (`self.Destination`)))
  (if (`KismetArrayLibrary.Array_IsValidIndex` (`self.BoatQueue`))
    (bind _returnvalue_2 (`|SpawnActorFromClass` (`|GetArrayItem` (`self.BoatQueue`)) (`KismetMathLibrary.MakeTransform` (`KismetMathLibrary.MakeVector` (.x (.location _returnvalue)) (.y (.location _returnvalue)) (.z (.location _returnvalue))) (.rotation _returnvalue) (.scale _returnvalue)) "Undefined" "MultiplyWithRoot" null null))
    (`/Game/Blueprints/Core/BP_Boat.Move` _returnvalue_2 (`KismetMathLibrary.MakeVector` _destination_x _destination_y (.z (.location _returnvalue))))
    (`KismetArrayLibrary.Array_Remove` (`self.BoatQueue`))
    (return true)
    (else
      (return false))))

(fn `UserConstructionScript`)