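; Hidden platform actor that holds teleported units in formation, with a separate platform for each of up to four commanders.
; Construction script builds each platform's slot array from a formation center component and its children.
; Teleporting disables the unit's behaviour tree and its commander's selectability, then places the unit at the slot indexed by that platform's unit count.
; SelectPlatform matches the unit's commander to a platform, claiming the first free one for new commanders.
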(fn `Add Unit To Platform`
  (params (`Platform Number` :type Integer) (Unit :type "/Game/Blueprints/Core/Units/BP_Unit Object Reference"))
  (locals (`Unit Var` :type "/Game/Blueprints/Core/Units/BP_Unit Object Reference"))
  (set `local.Unit Var` Unit)
  (switch `int` `Platform Number`
    (:`1`
      (`KismetArrayLibrary.Array_Add` (`self.Position 1 Units`) (`local.Unit Var`)))
    (:`2`
      (`KismetArrayLibrary.Array_Add` (`self.Position 2 Units`) (`local.Unit Var`)))
    (:`3`
      (`KismetArrayLibrary.Array_Add` (`self.Position 3 Units`) (`local.Unit Var`)))
    (:`4`
      (`KismetArrayLibrary.Array_Add` (`self.Position 4 Units`) (`local.Unit Var`)))))

(fn `Select Platform`
  (params (Unit :type "/Game/Blueprints/Core/Units/BP_Unit Object Reference"))
  (returns (`Positions Array` :type "Array of SceneComponent Object Reference") (`Units Array` :type "Array of /Game/Blueprints/Core/Units/BP_Unit Object Reference") (`Platform Number` :type Integer))
  (locals (Commander :type "/Game/Blueprints/Core/Units/Commander/BP_Commander Object Reference") (IsCommander :type Boolean))
  (bind _asbp_commander (cast `/Game/Blueprints/Core/Units/Commander/BP_Commander` Unit)
    (:`then`
      (set `local.IsCommander` true)
      (set `local.Commander` _asbp_commander))
    (:`CastFailed`
      (set `local.Commander` (`/Game/Blueprints/Core/Units/BP_Unit.Commander` Unit))))
  (`/Engine/EditorBlueprintResources/StandardMacros.IsValid` (`self.Commander 1`)
    (:`Is Valid`
      (if (!= (`self.Commander 1`) (`local.Commander`))
        (`/Engine/EditorBlueprintResources/StandardMacros.IsValid` (`self.Commander 2`)
          (:`Is Valid`
            (if (!= (`self.Commander 2`) (`local.Commander`))
              (`/Engine/EditorBlueprintResources/StandardMacros.IsValid` (`self.Commander 3`)
                (:`Is Valid`
                  (if (!= (`self.Commander 3`) (`local.Commander`))
                    (`/Engine/EditorBlueprintResources/StandardMacros.IsValid` (`self.Commander 4`)
                      (:`Is Valid`
                        (if (not (!= (`self.Commander 4`) (`local.Commander`)))
                          (return (`self.PositionsArray 4`) (`self.Position 4 Units`) 4)))
                      (:`Is Not Valid`
                        (set `self.Commander 4` (`local.Commander`))
                        (set `self.Commander 1 Healing` (`local.IsCommander`))
                        (return (`self.PositionsArray 4`) (`self.Position 4 Units`) 4)))
                    (else
                      (return (`self.PositionsArray 3`) (`self.Position 3 Units`) 3))))
                (:`Is Not Valid`
                  (set `self.Commander 3` (`local.Commander`))
                  (set `self.Commander 1 Healing` (`local.IsCommander`))
                  (return (`self.PositionsArray 3`) (`self.Position 3 Units`) 3)))
              (else
                (return (`self.PositionsArray 2`) (`self.Position 2 Units`) 2))))
          (:`Is Not Valid`
            (set `self.Commander 2` (`local.Commander`))
            (set `self.Commander 1 Healing` (`local.IsCommander`))
            (return (`self.PositionsArray 2`) (`self.Position 2 Units`) 2)))
        (else
          (return (`self.PositionsArray 1`) (`self.Position 1 Units`) 1))))
    (:`Is Not Valid`
      (set `self.Commander 1` (`local.Commander`))
      (set `self.Commander 1 Healing` (`local.IsCommander`))
      (return (`self.PositionsArray 1`) (`self.Position 1 Units`) 1))))

(fn `Teleport Onto Platform`
  (params (Unit :type "/Game/Blueprints/Core/Units/BP_Unit Object Reference"))
  (bind (_positions_array _units_array _platform_number) (`self.Select Platform` Unit))
  (`/Game/Blueprints/Core/Units/BP_Unit.Enable Disable Behaviour Tree` Unit false)
  (`self.K2_SetActorLocation` Unit (`SceneComponent.K2_GetComponentLocation` (`|GetArrayItem` _positions_array (`KismetArrayLibrary.Array_Length` _units_array))) false true)
  (set `/Game/Blueprints/Core/Units/Commander/BP_Commander.Can Be Selected` false (`/Game/Blueprints/Core/Units/BP_Unit.Commander` Unit))
  (`self.Add Unit To Platform` _platform_number Unit))

(fn `UserConstructionScript`
  (bind _output_get (set `self.PositionsArray 1` (`SceneComponent.GetChildrenComponents` (`self.FormationPositiosCenter1`) false)))
  (`KismetArrayLibrary.Array_Add` _output_get (`self.FormationPositiosCenter1`))
  (bind _output_get_2 (set `self.PositionsArray 2` (`SceneComponent.GetChildrenComponents` (`self.FormationPositiosCenter2`) false)))
  (`KismetArrayLibrary.Array_Add` _output_get_2 (`self.FormationPositiosCenter2`))
  (bind _output_get_3 (set `self.PositionsArray 3` (`SceneComponent.GetChildrenComponents` (`self.FormationPositiosCenter3`) false)))
  (`KismetArrayLibrary.Array_Add` _output_get_3 (`self.FormationPositiosCenter3`))
  (bind _output_get_4 (set `self.PositionsArray 4` (`SceneComponent.GetChildrenComponents` (`self.FormationPositiosCenter4`) false)))
  (`KismetArrayLibrary.Array_Add` _output_get_4 (`self.FormationPositiosCenter4`)))