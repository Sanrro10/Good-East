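; BP_HouseBig is the big house variant of a parent house Blueprint, overriding its highlight and ruined visuals for a mesh with two material slots.
; Highlight House applies the selection material to both slots when a valid Commander can heal and the house is selectable, and restores the original material when the Commander is invalid.
; Set Ruined House runs the parent logic, then puts the burned material on the second slot.
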(fn `Highlight House`
  (params (Commander :type "/Game/Blueprints/Core/Units/Commander/BP_Commander Object Reference"))
  (`/Engine/EditorBlueprintResources/StandardMacros.IsValid` Commander
    (:`Is Valid`
      (if (and (`/Game/Blueprints/Core/Units/Commander/BP_Commander.Get Can Heal` Commander) (`self.Get Can Be Selected`))
        (`PrimitiveComponent.SetMaterial` (`self.StaticMesh`) 0 (`self.SelectionMaterial`))
        (`PrimitiveComponent.SetMaterial` (`self.StaticMesh`) 1 (`self.SelectionMaterial`))))
    (:`Is Not Valid`
      (`PrimitiveComponent.SetMaterial` (`self.StaticMesh`) 0 (`self.OriginalMaterial`))
      (`PrimitiveComponent.SetMaterial` (`self.StaticMesh`) 1 (`self.OriginalMaterial`)))))

(fn `Set Ruined House`
  (`parent.Set Ruined House`)
  (`PrimitiveComponent.SetMaterial` (`self.StaticMesh`) 1 "/Game/Art/Materials/M_BurnedHouse.M_BurnedHouse"))

(fn `UserConstructionScript`
  (`parent.UserConstructionScript`))