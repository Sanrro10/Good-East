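; BP_House is a defense-game building that shelters allied units for healing and can be burned down by attackers.
; It registers with GM_DefenseGame, whose events drive selection highlighting and a victory coin widget for surviving houses.
; Units targeting its tile enter, update a healing progress widget, and respawn at the door on a looping timer.
; Queued attackers burn it sequentially, escalating fire, smoke and audio until it becomes a ruin.
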(event `self.ReceiveBeginPlay`
  (bind _asgm_defense_game (cast `/Game/Blueprints/Core/GM_DefenseGame` (`GameplayStatics.GetGameMode`)))
  (bind _output_get (set `self.GM Defense Game` _asgm_defense_game))
  (`/Game/Blueprints/Core/GM_DefenseGame.Add House` _output_get self)
  (add `/Game/Blueprints/Core/GM_DefenseGame.ShowTiles` (`self.GM Defense Game`) (delegate `ChangeMaterialToSelect`))
  (add `/Game/Blueprints/Core/GM_DefenseGame.HideTiles` (`self.GM Defense Game`) (delegate `ChangeMaterialToOriginal`))
  (add `/Game/Blueprints/Core/GM_DefenseGame.OnVictory` (`self.GM Defense Game`) (delegate `Event Show Coins Widget`))
  (bind _aswbp_healing_progress (cast `/Game/Blueprints/Widgets/InGameWidgets/WBP_HealingProgress` (`WidgetComponent.GetWidget` (`self.Healing Widget`))))
  (bind _output_get_2 (set `self.Healing Progress Widget` _aswbp_healing_progress))
  (`/Game/Blueprints/Widgets/InGameWidgets/WBP_HealingProgress.Initialize` _output_get_2 9)
  (`KismetSystemLibrary.DelayUntilNextTick`)
  (set `self.Hidden Platform` (`/Game/Blueprints/Core/GM_DefenseGame.HiddenPlatform` (`self.GM Defense Game`))))

(event `Event Show Coins Widget`
  (if (not (`self.Get Is Destroyed`))
    (bind _aswbp_coins (cast `/Game/Blueprints/Widgets/InGameWidgets/WBP_Coins` (`WidgetComponent.GetWidget` (`self.Coins Widget`))))
    (`/Game/Blueprints/Widgets/InGameWidgets/WBP_Coins.Initialize Widget` _aswbp_coins (`self.Gold`))))

(event `ChangeMaterialToSelect`
  (params (Commander :type "/Game/Blueprints/Core/Units/Commander/BP_Commander Object Reference"))
  (`self.Highlight House` Commander))

(event `ChangeMaterialToOriginal`
  (if (`self.Get Is Destroyed`)
    (`PrimitiveComponent.SetMaterial` (`self.StaticMesh`) 0 "/Game/Art/Materials/M_BurnedHouse.M_BurnedHouse")
    (`PrimitiveComponent.SetMaterial` (`self.StaticMesh`) 1 "/Game/Art/Materials/M_BurnedHouse.M_BurnedHouse")
    (else
      (`self.Highlight House` null))))

(event `UnitTryEnterHouse`
  (params (Unit :type "/Game/Blueprints/Core/Units/BP_Unit Object Reference"))
  (`self.AllyEnterHouseTrigger` Unit))

(event `self.Box.OnComponentBeginOverlap`
  (params (OverlappedComponent :type "PrimitiveComponent Object Reference") (OtherActor :type "Actor Object Reference") (OtherComp :type "PrimitiveComponent Object Reference") (OtherBodyIndex :type Integer) (bFromSweep :type Boolean) (SweepResult :type "HitResult Structure (by ref)"))
  (`self.AllyEnterHouseTrigger` OtherActor))

(event `Event Respawn Unit`
  (bind _units_resting (`self.Units Resting`))
  (bind _returnvalue (`SceneComponent.K2_GetComponentToWorld` (`self.DoorBillboard`)))
  (bind _output (`|GetArrayItem` _units_resting))
  (if (`KismetArrayLibrary.Array_IsNotEmpty` _units_resting)
    (`/Game/Blueprints/Core/BP_HiddenPlatform.Remove Unit From Platform` (`self.Hidden Platform`) _output)
    (`self.K2_SetActorLocationAndRotation` _output (`KismetMathLibrary.MakeVector` (.x (.location _returnvalue)) (.y (.location _returnvalue)) (+ (.z (.location _returnvalue)) 85.0)) (.rotation _returnvalue) false true)
    (`/Game/Blueprints/Core/Units/BP_AlliedUnit.Reactivate Unit After Healing` _output (`/Game/Blueprints/Core/BP_Tile.RespawnTile` (`self.House Tile`)))
    (`KismetArrayLibrary.Array_Remove` (`self.Units Resting`))
    (else
      (`KismetSystemLibrary.K2_ClearAndInvalidateTimerHandle` (stale `Event Start Respawning Units` _returnvalue))
      (`KismetSystemLibrary.Delay` 2.0)
      (set `self.IsAccesible` true))))

(event `Event Start Respawning Units`
  (set `self.IsAccesible` false)
  (bind _commander (`/Game/Blueprints/Core/BP_Tile.Commander` (`/Game/Blueprints/Core/BP_Tile.RespawnTile` (`self.House Tile`)))
    (:`then`
      (`/Game/Blueprints/Core/Units/Commander/BP_Commander.RepositionToAdjacentTile` _commander null null))
    (:`else`
      _))
  (bind _returnvalue (`KismetSystemLibrary.K2_SetTimerDelegate` (delegate `Event Respawn Unit`) 0.5 true)))

(event `Add Attacking Unit`
  (params (Attacker :type "/Game/Blueprints/Core/Units/BP_EnemyUnit Object Reference (by ref)"))
  (`KismetArrayLibrary.Array_AddUnique` (`self.Attackers`) Attacker)
  (if (not (`self.Being Attacked`))
    (set `self.Being Attacked` true)
    (`self.Receive Attack`)))

(fn `Add Healing Unit`
  (params (Unit :type "/Game/Blueprints/Core/Units/BP_AlliedUnit Object Reference (by ref)"))
  (`KismetArrayLibrary.Array_AddUnique` (`self.Units Resting`) Unit)
  (if (not (`/Game/Blueprints/Core/Units/BP_Unit.GetIsDamaged` Unit))
    (`self.Progress Healing Widget`)))

(fn `Get Can Be Selected`
  (returns (Empty :type Boolean))
  (return (and (`KismetArrayLibrary.Array_IsEmpty` (`self.Units Resting`)) (`self.IsAccesible`) (not (`self.Get Is Destroyed`)))))

(fn `Get Is Destroyed`
  (returns (Destroyed :type Boolean))
  (return (or (`self.Destroyed`) (<= (`self.Health Points`) 0))))

(fn `GetDoorPosition`
  (returns (ReturnValue :type "Vector Structure"))
  (return (`SceneComponent.K2_GetComponentLocation` (`self.DoorBillboard`))))

(fn `Highlight House`
  (params (Commander :type "/Game/Blueprints/Core/Units/Commander/BP_Commander Object Reference"))
  (`/Engine/EditorBlueprintResources/StandardMacros.IsValid` Commander
    (:`Is Valid`
      (if (and (`/Game/Blueprints/Core/Units/Commander/BP_Commander.Get Can Heal` Commander) (`self.Get Can Be Selected`))
        (for _index (range (+ (`PrimitiveComponent.GetNumMaterials` (`self.StaticMesh`)) 1))
          (`PrimitiveComponent.SetMaterial` (`self.StaticMesh`) _index (`self.SelectionMaterial`)))))
    (:`Is Not Valid`
      (for _index_2 (range (+ (`PrimitiveComponent.GetNumMaterials` (`self.StaticMesh`)) 1))
        (`PrimitiveComponent.SetMaterial` (`self.StaticMesh`) _index_2 (`self.OriginalMaterial`))))))

(fn `Progress Healing Widget`
  (`/Game/Blueprints/Widgets/InGameWidgets/WBP_HealingProgress.Add Progress ` (`self.Healing Progress Widget`))
  (return))

(fn `Receive Attack`
  (bind _attackers (`self.Attackers`))
  (bind _output (`|GetArrayItem` _attackers))
  (if (`KismetArrayLibrary.Array_IsNotEmpty` _attackers)
    (`/Engine/EditorBlueprintResources/StandardMacros.IsValid` _output
      (:`Is Valid`
        (`/Game/Blueprints/Core/Units/BP_EnemyUnit.Burn House` _output self)
        (`KismetArrayLibrary.Array_Remove` _attackers))
      (:`Is Not Valid`
        (`KismetArrayLibrary.Array_Remove` (`self.Attackers`))
        (`self.Receive Attack`)))
    (else
      (set `self.Being Attacked` false))))

(fn `Receive Damage`
  (bind _health_points (`self.Health Points`))
  ;[0.1848 0.86 1] If the house has no more hp left
  (`/Engine/EditorBlueprintResources/StandardMacros.DecrementInt` _health_points
    (:`  `
      (if (<= _health_points 0)
        (`/Game/Blueprints/Core/GM_DefenseGame.Remove House` (`self.GM Defense Game`) self)
        (set `self.Destroyed` true)
        (`self.Set Ruined House`)
        (else
          (`self.StartFires` (/ (`self.Health Points`) (`self.Initial Health Points`)))
          (`self.Receive Attack`))))))

(fn `Reset Healing Widget Progress`
  (`/Game/Blueprints/Widgets/InGameWidgets/WBP_HealingProgress.Reset Progress` (`self.Healing Progress Widget`)))

(fn `Set Healing Widget Visible`
  (params (Visible :type Boolean))
  (`SceneComponent.SetVisibility` (`self.Healing Widget`) Visible true))

(fn `Set Ruined House`
  (`ActorComponent.Deactivate` (`self.FireParticleSystem`))
  (`ActorComponent.Deactivate` (`self.FireParticleSystem1`))
  (`ActorComponent.Deactivate` (`self.FireParticleSystem2`))
  ;[0 0.3437 1] Audio
  (`AudioComponent.Stop` (`self.FireAudio`))
  (`/Game/Blueprints/Core/GM_DefenseGame.Remove House` (`self.GM Defense Game`) self)
  (`self.Set Healing Widget Visible` false)
  ;[0.4766 0 1] Changes Material
  (`PrimitiveComponent.SetMaterial` (`self.StaticMesh`) 0 "/Game/Art/Materials/M_BurnedHouse.M_BurnedHouse")
  (if (== (`PrimitiveComponent.GetNumMaterials` (`self.StaticMesh`)) 2)
    (`PrimitiveComponent.SetMaterial` (`self.StaticMesh`) 1 "/Game/Art/Materials/M_BurnedHouse.M_BurnedHouse")))

(fn `StartFires`
  (params (HouseLifePer :type "Float (double-precision)"))
  (locals (LifePer :type "Float (double-precision)"))
  (bind _fireparticlesystem (`self.FireParticleSystem`))
  (bind _fireparticlesystem2 (`self.FireParticleSystem2`))
  (bind _fireparticlesystem1 (`self.FireParticleSystem1`))
  (set `local.LifePer` HouseLifePer)
  (if (>= (`local.LifePer`) 0.666667)
    ;[1 0.4657 0.3021] >2/3
    (if (not (`ActorComponent.IsActive` _fireparticlesystem))
      (`ActorComponent.Activate` _fireparticlesystem true)
      (`ActorComponent.Activate` (`self.SmokeParticleSystem3`) true)
      (`ActorComponent.Activate` (`self.SmokeParticleSystem4`) true)
      ;[1 0.6797 0] Audio
      (`AudioParameterControllerInterface.SetIntParameter` (`self.FireAudio`) "Fire" 0)
      (`AudioComponent.Play` (`self.FireAudio`) 0.0))
    (else
      ;[1 0.375 0.7852] <2/3
      (if (>= (`local.LifePer`) 0.333333)
        (if (not (`ActorComponent.IsActive` _fireparticlesystem1))
          (`ActorComponent.Activate` _fireparticlesystem1 true)
          (`ActorComponent.Activate` (`self.SmokeParticleSystem5`) true)
          (`ActorComponent.Activate` (`self.SmokeParticleSystem6`) true)
          (`AudioParameterControllerInterface.SetIntParameter` (`self.FireAudio`) "Fire" 1)
          (`AudioComponent.Play` (`self.FireAudio`) 0.0))
        (else
          ;[0.2656 1 0.6385] <1/3
          (if (not (`ActorComponent.IsActive` _fireparticlesystem2))
            (`ActorComponent.Activate` _fireparticlesystem2 true)
            (`ActorComponent.Activate` (`self.SmokeParticleSystem7`) true)
            (`ActorComponent.Activate` (`self.SmokeParticleSystem8`) true)
            (`AudioParameterControllerInterface.SetIntParameter` (`self.FireAudio`) "Fire" 2)
            (`AudioComponent.Play` (`self.FireAudio`) 0.0)))))))

(fn `UserConstructionScript`
  (set `self.Health Points` (`self.Initial Health Points`))
  (set `self.OriginalMaterial` (`PrimitiveComponent.GetMaterial` (`self.StaticMesh`) 0)))