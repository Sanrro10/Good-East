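; BP_Torch is a thrown fire projectile that enemy units use to burn houses.
; ActivateTorch sets a homing target, launches the torch on a steep gravity-affected arc and starts its fire particles.
; Overlapping a BP_House makes an enemy-unit instigator deal burn damage, then destroys the torch.
; Without a valid instigator it is destroyed without damage, and DestroyTorch allows direct removal.
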(event `self.StaticMesh.OnComponentBeginOverlap`
  (params (OverlappedComponent :type "PrimitiveComponent Object Reference") (OtherActor :type "Actor Object Reference") (OtherComp :type "PrimitiveComponent Object Reference") (OtherBodyIndex :type Integer) (bFromSweep :type Boolean) (SweepResult :type "HitResult Structure (by ref)"))
  (bind _returnvalue (`self.GetInstigator`))
  (cast `/Game/Blueprints/Core/Houses/BP_House` OtherActor)
  (`/Engine/EditorBlueprintResources/StandardMacros.IsValid` _returnvalue
    (:`Is Valid`
      (bind _asbp_enemy_unit (cast `/Game/Blueprints/Core/Units/BP_EnemyUnit` _returnvalue))
      (`/Game/Blueprints/Core/Units/BP_EnemyUnit.House Burn Deal Damage` _asbp_enemy_unit))
    (:`Is Not Valid`
      _))
  (`self.K2_DestroyActor`))

(fn `Activate Torch`
  (params (`Target Component` :type "SceneComponent Object Reference"))
  (bind _projectilemovement (`self.ProjectileMovement`))
  (set `ProjectileMovementComponent.HomingTargetComponent` `Target Component` _projectilemovement)
  (set `ProjectileMovementComponent.ProjectileGravityScale` 1.0 _projectilemovement)
  (`ProjectileMovementComponent.SetVelocityInLocalSpace` _projectilemovement (400.0 0.0 7000.0))
  (set `ProjectileMovementComponent.bRotationFollowsVelocity` true _projectilemovement)
  (`PrimitiveComponent.SetEnableGravity` (`self.StaticMesh`) true)
  (`ActorComponent.Activate` (`self.FireParticleSystem`) false)
  (set `self.Active` true))

(fn `DestroyTorch`
  (`self.K2_DestroyActor`))

(fn `UserConstructionScript`)