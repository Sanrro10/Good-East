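; BP_Arrow is an arrow projectile, with optional homing, that damages and knocks back units of the opposing side.
; Collision stays off until projectile movement activates, with overlaps generated only if IsFailed is false.
; A unit overlap with a bone attaches and stops the arrow; without one, only overlaps and homing switch off.
; A blocking hit freezes it and its VFX; the line trace for HitLocation is disconnected.
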(event `self.Box.OnComponentBeginOverlap`
  (params (OverlappedComponent :type "PrimitiveComponent Object Reference") (OtherActor :type "Actor Object Reference") (OtherComp :type "PrimitiveComponent Object Reference") (OtherBodyIndex :type Integer) (bFromSweep :type Boolean) (SweepResult :type "HitResult Structure (by ref)"))
  (bind _asbp_unit (cast `/Game/Blueprints/Core/Units/BP_Unit` OtherActor))
  (`self.Enemy Hit` _asbp_unit OtherComp (`SkinnedMeshComponent.GetBoneName` (`Character.Mesh` _asbp_unit) OtherBodyIndex)))

(event `self.Box.OnComponentHit`
  (params (HitComponent :type "PrimitiveComponent Object Reference") (OtherActor :type "Actor Object Reference") (OtherComp :type "PrimitiveComponent Object Reference") (NormalImpulse :type "Vector Structure") (Hit :type "HitResult Structure (by ref)"))
  (`self.SetActorEnableCollision` false)
  (`MovementComponent.StopMovementImmediately` (`self.ProjectileMovement`))
  (`SceneComponent.SetMobility` (`self.StaticMesh`) "Static")
  (`ActorComponent.Deactivate` (`self.ProjectileMovement`))
  ;[1 0 0.9609] VFX
  (`ActorComponent.Deactivate` (`self.ArrowTip`))
  (`ActorComponent.Deactivate` (`self.ArrowTrail`))
  (`KismetSystemLibrary.PrintString` "GROUND HIT"))

(event `self.ProjectileMovement.OnComponentActivated`
  (params (Component :type "ActorComponent Object Reference") (bReset :type Boolean))
  (set `PrimitiveComponent.bGenerateOverlapEvents` (not (`self.Is Failed`)) (`self.Box`))
  (`self.SetActorEnableCollision` true))

(fn `Enemy Hit`
  (params (`Enemy Hit` :type "/Game/Blueprints/Core/Units/BP_Unit Object Reference") (`Component Hit` :type "PrimitiveComponent Object Reference") (`Bone Name` :type Name))
  (locals (`Hit Location` :type "Vector Structure" :default (0.0 0.0 0.0)) (`Hit Normal` :type "Vector Structure") (`Target Bone` :type Name))
  (bind _projectilemovement (`self.ProjectileMovement`))
  (if (!= (`/Game/Blueprints/Core/Units/BP_Unit.isEnemy` `Enemy Hit`) (`self.Is Enemy`))
    (`/Game/Blueprints/Core/Units/BP_Unit.Event Receive Damage` (`local.Enemy Hit`) (`self.Damage`) (* (`SceneComponent.GetForwardVector` (`self.Arrow`)) (`self.Knock Back Strength`)))
    ;[0.1719 1 0] Deprecated
    (if (== (`local.Bone Name`) "None")
      (set `PrimitiveComponent.bGenerateOverlapEvents` false (`self.Box`))
      (set `ProjectileMovementComponent.bIsHomingProjectile` false (`self.ProjectileMovement`))
      (else
        (`self.SetActorEnableCollision` false)
        (`KismetSystemLibrary.PrintString` (`KismetStringLibrary.Concat_StrStr` "ATTACHED TO " (`KismetSystemLibrary.GetDisplayName` (`local.Enemy Hit`)) (`KismetStringLibrary.Conv_NameToString` `Bone Name`)))
        (`self.K2_AttachToComponent` (`local.Component Hit`) `Bone Name` "SnapToTarget" "KeepWorld" "KeepWorld")
        (`self.K2_SetActorLocation` (+ (`local.Hit Location`) (* 5.0 (`SceneComponent.GetForwardVector` (`self.Arrow`)))))
        (set `ProjectileMovementComponent.bIsHomingProjectile` false _projectilemovement)
        (`MovementComponent.StopMovementImmediately` _projectilemovement)
        (`ActorComponent.Deactivate` _projectilemovement)
        (`self.SetActorEnableCollision` false)
        ;[1 0 0.9609] VFX
        (`ActorComponent.Deactivate` (`self.ArrowTip`))
        (`ActorComponent.Deactivate` (`self.ArrowTrail`))))))

(fn `UserConstructionScript`
  (`self.SetActorEnableCollision` false))