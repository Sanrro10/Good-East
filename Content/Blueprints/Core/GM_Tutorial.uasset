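; GM_Tutorial is the tutorial game mode, layering on-screen hints over its parent's level start and enemy death logic.
; On level start it shows a WBP_Tutorial widget with unit movement text, runs the parent logic, then adds a camera rotation widget after a short delay.
; Its EnemyDead override calls the parent, counts kills, and displays a further tutorial widget when the counter check matches a fixed threshold.
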(event `self.Event Start Level `
  (bind _returnvalue (`|CreateWidget` "/Game/Blueprints/Widgets/SubMenus/WBP_Tutorial.WBP_Tutorial_C"))
  (set `/Game/Blueprints/Widgets/SubMenus/WBP_Tutorial.TutorialText` (`self.Unit Movement Tutorial Text`) _returnvalue)
  (`UserWidget.AddToViewport` _returnvalue 0)
  (`parent.Event Start Level `)
  (`KismetSystemLibrary.Delay` 3.0)
  (bind _returnvalue_2 (`|CreateWidget` "/Game/Blueprints/Widgets/SubMenus/WBP_Tutorial.WBP_Tutorial_C"))
  (set `/Game/Blueprints/Widgets/SubMenus/WBP_Tutorial.TutorialText` (`self.Camera Rotation Tutorial Text`) _returnvalue_2)
  (`UserWidget.AddToViewport` _returnvalue_2 0))

(fn `Enemy Dead`
  (params (Enemy :type "/Game/Blueprints/Core/Units/BP_EnemyUnit Object Reference (by ref)"))
  (locals (`Tutorial Text` :type Text :default "NSLOCTEXT(\"\", \"A496ED4D4738BAAB3B46DCA59017BBD0\", \"You can heal a unit by selecting it and clicking on a house.\")"))
  (`parent.Enemy Dead` Enemy)
  (bind _result (`/Engine/EditorBlueprintResources/StandardMacros.IncrementInt` (`self.Enemies Killed`))
    (:`  `
      (if (== _result 4)
        (bind _returnvalue (`|CreateWidget` "/Game/Blueprints/Widgets/SubMenus/WBP_Tutorial.WBP_Tutorial_C"))
        (set `/Game/Blueprints/Widgets/SubMenus/WBP_Tutorial.TutorialText` (`local.Tutorial Text`) _returnvalue)
        (`UserWidget.AddToViewport` _returnvalue 0)
        (else
          (return))))))

(fn `UserConstructionScript`
  (`parent.UserConstructionScript`))