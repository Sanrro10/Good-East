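; BP_Grid is an actor that builds a square field of BP_Tile actors, spaced 400 units apart around the world origin.
; Its construction script compares Size to PreviousSize, calling SpawnTiles on growth and DespawnTiles otherwise.
; A location-keyed Tiles map prevents duplicate spawns and supplies the tiles to destroy.
; DespawnTiles loops only from Size to PreviousSize per axis, so it does not cover the whole removed border.
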(event `self.ReceiveBeginPlay`)

(fn `DespawnTiles`
  (locals (SpawnLocation :type "Vector Structure"))
  (bind (_spawnlocation_x _spawnlocation_y) (`KismetMathLibrary.BreakVector` (`local.SpawnLocation`)))
  (bind (_value _returnvalue) (`BlueprintMapLibrary.Map_Find` (`self.Tiles`) (`local.SpawnLocation`)))
  (bind _returnvalue_2 (`KismetMathLibrary.Conv_IntToDouble` (* (`self.Previous Size`) -400)))
  (set `local.SpawnLocation` (`KismetMathLibrary.MakeVector` _returnvalue_2 _returnvalue_2))
  (for _ (range (`self.Size`) (+ (`self.Previous Size`) 1))
    (for _ (range (`self.Size`) (+ (`self.Previous Size`) 1))
      (if _returnvalue
        (`self.K2_DestroyActor` _value)
        (`BlueprintMapLibrary.Map_Remove` (`self.Tiles`) (`local.SpawnLocation`))
        (set `local.SpawnLocation` (+ (`local.SpawnLocation`) (400.0 0.0 0.0)))))
    (set `local.SpawnLocation` (`KismetMathLibrary.MakeVector` (`KismetMathLibrary.Conv_IntToDouble` (* (`self.Size`) -400)) (+ _spawnlocation_y 400.0)))))

(fn `Spawn Tiles`
  (locals (SpawnLocation :type "Vector Structure" :default (0.0 0.0 0.0)) (`X Value` :type Integer) (`Y Value` :type Integer))
  (bind _size (`self.Size`))
  (bind _returnvalue (* _size -1))
  (set `local.SpawnLocation` (`KismetMathLibrary.MakeVector` 0.0))
  (for _index (range _returnvalue (+ _size 1))
    (set `local.X Value` _index)
    (for _index_2 (range _returnvalue (+ _size 1))
      (set `local.Y Value` _index_2)
      (set `local.SpawnLocation` (`KismetMathLibrary.MakeVector` (* (`local.X Value`) 400.0) (* (`local.Y Value`) 400.0)))
      (if (not (`BlueprintMapLibrary.Map_Contains` (`self.Tiles`) (`local.SpawnLocation`)))
        (bind _returnvalue_2 (`|SpawnActorFromClass` "/Game/Blueprints/Core/BP_Tile.BP_Tile_C" (`KismetMathLibrary.MakeTransform` (`local.SpawnLocation`)) "AlwaysSpawn" "MultiplyWithRoot" self null))
        (`SceneComponent.SetVisibility` (`/Game/Blueprints/Core/BP_Tile.Grid` _returnvalue_2) true false)
        (`BlueprintMapLibrary.Map_Add` (`self.Tiles`) (`local.SpawnLocation`) _returnvalue_2)))))

(fn `UserConstructionScript`
  (if (> (`self.Size`) (`self.Previous Size`))
    (`self.Spawn Tiles`)
    (else
      (`self.DespawnTiles`)))
  (set `self.Previous Size` (`self.Size`)))