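; BP_Tile is an environment tile actor that displays either a grass or a water static mesh.
; The Construction Script picks the mesh from the Type enum: the first value gives grass, while every other value gives water.
; The event graph has no logic, and its click event is an empty stub.
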(event `self.ReceiveActorOnClicked`
  (params (ButtonPressed :type "Key Structure")))

(fn `UserConstructionScript`
  (locals (SelectedStaticMesh :type "StaticMesh Object Reference"))
  (if (`|EnumEquality` (`self.Type`) "NewEnumerator0")
    (`StaticMeshComponent.SetStaticMesh` (`self.StaticMesh`) "/Game/Assets/PolygonKnights/Meshes/Environments/SM_Env_Tile_Grass_01.SM_Env_Tile_Grass_01")
    (elif (`|EnumEquality` (`self.Type`) "NewEnumerator1")
      (`StaticMeshComponent.SetStaticMesh` (`self.StaticMesh`) "/Game/Assets/PolygonKnights/Meshes/Environments/SM_Env_Tile_Water_01.SM_Env_Tile_Water_01")
      (else
        (`StaticMeshComponent.SetStaticMesh` (`self.StaticMesh`) "/Game/Assets/PolygonKnights/Meshes/Environments/SM_Env_Tile_Water_01.SM_Env_Tile_Water_01")))))