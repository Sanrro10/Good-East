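; BP_Camera is a player-controlled camera for the defense game that supports rotation and zoom through Enhanced Input.
; BeginPlay registers the default mapping context with the local DefenseGamePlayerController's input subsystem.
; The rotate action adds half its value to actor yaw, while the zoom action shifts the camera's field of view within clamped limits.
; The construction script sets a fixed starting rotation and leaves location at the default input.
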(event `self.ReceiveBeginPlay`
  (bind _asdefense_game_player_controller (cast `DefenseGamePlayerController` (`GameplayStatics.GetPlayerController` 0)))
  (bind _returnvalue (pcsubsystem `EnhancedInputLocalPlayerSubsystem` _asdefense_game_player_controller))
  (`/Engine/EditorBlueprintResources/StandardMacros.IsValid` _returnvalue
    (:`Is Valid`
      (`EnhancedInputSubsystemInterface.AddMappingContext` _returnvalue "/Game/Input/IMC_Default.IMC_Default" 0 (struct)))))

(event `EnhancedInput|/Game/Input/Actions/IA_RotateCamera`
  (params (ActionValue :type "Float (double-precision)") (ElapsedSeconds :type "Float (double-precision)") (TriggeredSeconds :type "Float (double-precision)") (InputAction :type "InputAction Object Reference" :default "/Game/Input/Actions/IA_RotateCamera.IA_RotateCamera"))
  (bind (_returnvalue_roll _returnvalue_pitch _returnvalue_yaw) (`KismetMathLibrary.BreakRotator` (`self.K2_GetActorRotation`)))
  (:`Triggered`
    (`self.K2_SetActorRotation` (`KismetMathLibrary.MakeRotator` _returnvalue_roll _returnvalue_pitch (+ _returnvalue_yaw (/ ActionValue 2.0))))))

(event `EnhancedInput|/Game/Input/Actions/IA_ZoomCamera`
  (params (ActionValue :type "Float (double-precision)") (ElapsedSeconds :type "Float (double-precision)") (TriggeredSeconds :type "Float (double-precision)") (InputAction :type "InputAction Object Reference" :default "/Game/Input/Actions/IA_ZoomCamera.IA_ZoomCamera"))
  (bind _camera (`self.Camera`))
  (bind _returnvalue (+ ActionValue (`CameraComponent.FieldOfView` (`self.Camera`))))
  (:`Triggered`
    (if (< _returnvalue 40.0)
      (`CameraComponent.SetFieldOfView` (`self.Camera`) 40.0)
      (elif (> _returnvalue 120.0)
        (`CameraComponent.SetFieldOfView` _camera 120.0)
        (else
          (`CameraComponent.SetFieldOfView` _camera _returnvalue))))))

(fn `UserConstructionScript`
  (`self.K2_SetActorLocationAndRotation` (0.0 0.0 0.0) (struct :`Pitch` -90.0)))